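; Demonic bow item that needs no ammunition, always firing one fixed ammo type, and cannot leave its owner's backpack, equipment or shortcut bar.
; While equipped, a looping timer keeps the wielder's corruption at or above a set minimum.
; Kill XP signals restore durability scaled by the victim's max health.
; At zero durability, the bow is deleted from the owner's inventory.
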(event `self.OnUnEquip`
  (params (owner :type "Character Object Reference"))
  (`parent.OnUnEquip` owner)
  (`KismetSystemLibrary.K2_ClearAndInvalidateTimerHandle` (`self.CorruptionTimer`)))

(event `self.OnEquip`
  (params (owner :type "Character Object Reference"))
  (`parent.OnEquip` owner)
  (set `self.Owner` owner)
  (add `/Game/Characters/BaseBPCombat.SignalGiveKillXP` (cast `/Game/Characters/BaseBPCombat` owner :!pure true) (`|CreateDelegate` :!event `Event PlayerKilledSomething`))
  (`self.SetAmmunition` 43002)
  (add `self.SignalFloatStatChanged` (delegate `Durability`))
  (bind _returnvalue (`KismetSystemLibrary.K2_SetTimerDelegate` (delegate `AddCorruption`) 3.0 true))
  (set `self.CorruptionTimer` _returnvalue)
  (`self.AddCorruption`))

(event `AddCorruption`
  (bind _returnvalue (`Actor.GetComponentByClass` (`self.Owner`) "/Game/Systems/BPEnergyReceiver.BPEnergyReceiver_C"))
  (`/Engine/EditorBlueprintResources/StandardMacros.IsValid` _returnvalue
    (:`Is Valid`
      (if (< (`EnergyReceiverComponent.GetEnergy` _returnvalue "EnergyType_Corruption") (`self.NewCorruptionAmount`))
        (`EnergyReceiverComponent.SetEnergy` _returnvalue "EnergyType_Corruption" (`self.NewCorruptionAmount`) 0.0)))))

(event `Durability` :!signature `self.SignalFloatStatChanged`
  (params (item :type "GameItem Object Reference") (statID :type "EItemFloatStatID Enum") (newValue :type "Float (double-precision)") (deltaValue :type "Float (double-precision)"))
  (if (and (`|EnumEquality` statID "CurrentDurability") (== newValue 0.0))
    (`ItemInventory.DeleteItemsByTemplate` (`self.GetOwnerInventory`) (`self.TemplateID`) "disappear" 99)))

(event `Event PlayerKilledSomething`
  (params (PlayerActor :type "Actor Object Reference") (KilledActor :type "Actor Object Reference") (FractionToReceive :type "Float (double-precision)"))
  (bind _asconan_character (cast `ConanCharacter` KilledActor))
  (`self.SetDurability` (`KismetMathLibrary.FClamp` (+ (* (`self.BaseRepairAmtPerKill`) (`KismetMathLibrary.FClamp` (`KismetMathLibrary.NormalizeToRange` (`KismetMathLibrary.Conv_IntToDouble` (`ConanCharacter.GetIntStat` _asconan_character "HealthMax" "Full")) 0.0 800.0) 0.0 2.0)) (`self.GetFloatStat` "CurrentDurability")) 0.0 (`self.GetFloatStat` "MaxDurability"))))

(fn `AllowsMoveTo`
  (params (srcIndex :type Integer) (targetInventory :type "ItemInventory Object Reference") (targetIndex :type Integer) (quantity :type Integer))
  (returns (ReturnValue :type Boolean))
  (bind _inventorytype (`ItemInventory.InventoryType` targetInventory))
  (return (and (or (`|EnumEquality` _inventorytype "Backpack") (`|EnumEquality` _inventorytype "Equipment") (`|EnumEquality` _inventorytype "ShortcutBar")) (== (`self.GetOwner`) (`ActorComponent.GetOwner` targetInventory)))))

(fn `CanItemBeDroppedOnItem`
  (params (droppedItem :type "GameItem Object Reference") (srcInventory :type "ItemInventory Object Reference") (srcIndex :type Integer))
  (returns (ReturnValue :type Boolean))
  (return false))

(fn `CanSetAmmo`
  (params (Item :type "GameItem Object Reference"))
  (returns (Result :type Boolean))
  (return false))

(fn `GetCompatibleAmmunition`
  (returns (CompatibleAmmunitionID :type Integer))
  (return 43002))

(fn `GetCompatibleAmmunitions`
  (returns (CompatibleAmmunitions :type "Array of Integer"))
  (return (`|MakeArray` 43002)))

(fn `GetDefaultAmmoFallbackID`
  (returns (DefaultAmmoFallbackID :type Integer))
  (return 43002))

(fn `GetLoadedAmmunitionTemplateID`
  (returns (ReturnValue :type Integer))
  (return 43002))

(fn `HasActiveAmmunition`
  (returns (HasLoadedAmmo :type Boolean))
  (`self.SetIntStat` "ActiveAmmunition" 43002)
  (return true))

(fn `IsDurabilityBarPrioritized`
  (returns (ReturnValue :type Boolean))
  (return true))

(fn `RequiresAmmunition`
  (returns (RequiresAmmo :type Boolean))
  (return false))
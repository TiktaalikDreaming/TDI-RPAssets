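; Triangle foundation building piece that extends its parent's placement check to require support beneath it.
; CanBePlaced box-traces vertically around Box1 for static ground, caching HasFoundLandscape, and sweeps CheckForFoundationBox downward for structures tagged Building.Foundation_Wedge.
; Either hit returns the parent's result; otherwise placement fails with a missing-landscape error.
; Off the server, loading skips these checks and relies on the parent result alone.
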(fn `CanBePlaced`
  (params (AttachTo :type "BuildableBase Object Reference") (InstanceIndex :type Integer))
  (returns (FailedMessage :type String) (ReturnValue :type "ECanBePlacedResult Enum"))
  (locals (HasFoundLandscape :type Boolean))
  (bind _box1 (`self.Box1`))
  (bind _returnvalue (`SceneComponent.K2_GetComponentLocation` _box1))
  (bind (_failedmessage _returnvalue_2) (`parent.CanBePlaced` AttachTo InstanceIndex))
  (if (`KismetSystemLibrary.IsServer`)
    (if (< (`KismetMathLibrary.Conv_ByteToInt` 0) (`KismetMathLibrary.Conv_ByteToInt` (enumliteral `ECanBePlacedResult` "Fail")))
      _
      (else
        (return _failedmessage _returnvalue_2)))
    (elif (`self.m_IsLoading`)
      (if (< (`KismetMathLibrary.Conv_ByteToInt` _returnvalue_2) (`KismetMathLibrary.Conv_ByteToInt` (enumliteral `ECanBePlacedResult` "Fail")))
        (return "" "Success")
        (else
          (return _failedmessage _returnvalue_2)))
      (else
        _)))
  (bind _outhits (`KismetSystemLibrary.BoxTraceMulti` (`KismetMathLibrary.MakeVector` (.x _returnvalue) (.y _returnvalue) (+ (.z _returnvalue) 128.0)) (`KismetMathLibrary.MakeVector` (.x _returnvalue) (.y _returnvalue) (- (.z _returnvalue) 32.0)) (`BoxComponent.BoxExtent` _box1) (`SceneComponent.K2_GetComponentRotation` _box1) "TraceTypeQuery1"))
  (bind _returnvalue_3 (`BuildableFunctionLibrary.HasStaticGroundInHitResults` _outhits))
  (set `local.HasFoundLandscape` _returnvalue_3)
  (bind _foundoverlaps (`/Game/Systems/Building/BuildingFunctionLibrary.CheckForOverlappingStructure` (`self.CheckForFoundationBox`) 32.0 (struct :`GameplayTags` (struct :`(TagName` "Building.Foundation_Wedge") :`(TagName` "Building.Pillar") :`(TagName` "Building.Ceiling_Wedge")))))
  (if (or _foundoverlaps (`local.HasFoundLandscape`))
    (return _failedmessage _returnvalue_2)
    (else
      (return (`KismetTextLibrary.Conv_TextToString` (`self.Error_CouldntFindLandscapeTriangles`)) "Fail"))))

(fn `UserConstructionScript`
  (`parent.UserConstructionScript`))
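; Placeable siege-defense cauldron that players load with ammo and tip to spawn a payload actor, then reset before reuse.
; Server-side interaction consumes ammo matched through a data table and toggles replicated HasFired, whose OnRep runs the fire or reverse timeline animating cauldron and lever.
; The fire timeline's event track spawns the payload on the server.
; Inventory changes recheck ammo, driving replicated IsBoiling for oil visibility and boiling sound.
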(event `FirePayload`
  (`|SpawnActorFromClass` (`self.CauldronAmmoClass`) (`KismetMathLibrary.MakeTransform` (+ (* (`self.GetActorUpVector` self) 64.0) (* (`self.GetActorRightVector` self) 64.0) (.location (`self.GetTransform`))) (.rotation (`self.GetTransform`)) (.scale (`self.GetTransform`))) "Undefined" "OverrideRootScale" null (`Controller.K2_GetPawn` (`self.Attackinstigator`))))

(event `self.ReceiveBeginPlay`
  (bind _placeableinventory (`self.PlaceableInventory`))
  (`parent.ReceiveBeginPlay`)
  (if (`KismetSystemLibrary.IsServer`)
    (add `ItemInventory.SignalItemAdded` _placeableinventory (delegate `ItemAdded`))
    (add `ItemInventory.SignalItemRemoved` _placeableinventory (delegate `ItemRemoved`))
    (add `ItemInventory.SignalItemFloatStatChanged` _placeableinventory (delegate `ItemChanged`))
    (`self.CheckForAmmoSound` 0)))

(event `ItemAdded`
  (params (index :type Integer) (item :type "GameItem Object Reference") (srcInventory :type "ItemInventory Object Reference") (srcIndex :type Integer))
  (`self.CheckForAmmoSound` 0 :!label _label))

(event `ItemRemoved`
  (params (index :type Integer) (item :type "GameItem Object Reference") (dstInventory :type "ItemInventory Object Reference") (dstIndex :type Integer))
  (goto _label))

(event `ItemChanged`
  (params (item :type "GameItem Object Reference") (statID :type "EItemFloatStatID Enum") (statValue :type "Float (double-precision)") (deltaValue :type "Float (double-precision)"))
  (goto _label))

(event `TriggerPayload`
  (`self.CheckForAmmoSound` 0)
  (if (`KismetSystemLibrary.IsServer`)
    (`self.FirePayload`)))

(event `PlayFiringAudio`
  (if (not (`KismetSystemLibrary.IsDedicatedServer`))
    (`ConanAudioComponent.FadeIn` (`self.FiringAudio`) 0.0 1.0 0.0)
    (`ConanAudioComponent.Play` (`self.LeverAudio`) 0.0 :!label _label_2)))

(event `FireSiegeEquipment`
  (`self.PlayFiringAudio`)
  (bind (_direction _cauldronrot) (`Timeline|Timeline_0` :!via `PlayFromStart`)
    (:`Update`
      (`SceneComponent.K2_SetRelativeRotation` (`self.Cauldron`) (* (`self.CauldronEndRotation`) _cauldronrot) false false)
      (`SceneComponent.K2_SetRelativeRotation` (`self.Lever`) (`KismetMathLibrary.ComposeRotators` (`self.DefaultLeverRot`) (* (`self.InteractHandleRot`) _cauldronrot)) false false))
    (:`Finished`
      (set `self.CanBeReversed` true))
    (:`PayloadTrigger`
      (`self.TriggerPayload`))))

(event `CheckForAmmoSound`
  (params (index :type Integer) (item :type "GameItem Object Reference") (srcInventory :type "ItemInventory Object Reference") (srcIndex :type Integer))
  (bind (_hasammo_ _cauldronammoclass _soundwhileincauldron) (`self.CheckAmmo` false))
  (set `self.BoilingSoundToPlay` _soundwhileincauldron)
  (set `self.IsBoiling` (and _hasammo_ (`self.isReady`))))

(event `PlayBoilingAmmoSound`
  (params (IsBoiling :type Boolean) (SoundWhileInCauldron :type "SoundCue Object Reference"))
  (bind _boilingsound (`self.BoilingSound`))
  (if (`KismetSystemLibrary.IsDedicatedServer`)
    _
    (elif IsBoiling
      (`ConanAudioComponent.Stop` _boilingsound)
      (`ConanAudioComponent.SetSound` _boilingsound SoundWhileInCauldron)
      (`ConanAudioComponent.FadeIn` _boilingsound 1.0 1.0 0.0)
      (`SceneComponent.SetVisibility` (`self.OilCylinder`) true false)
      (else
        (`ConanAudioComponent.FadeOut` _boilingsound 1.0 0.0)
        (`SceneComponent.SetVisibility` (`self.OilCylinder`) false false)))))

(event `PlayReverseAudio`
  (if (not (`KismetSystemLibrary.IsDedicatedServer`))
    (`ConanAudioComponent.FadeIn` (`self.ReverseAudio`) 0.0 1.0 0.0)
    (goto _label_2)))

(event `ReverseSiegeEquipment`
  (`self.PlayReverseAudio`)
  (`TimelineComponent.SetPlayRate` (`self.Timeline_1`) (`self.Reverse_PlayRate`))
  (bind (_direction _cauldronrot) (`Timeline|Timeline_1` :!via `ReverseFromEnd`)
    (:`Update`
      (`SceneComponent.K2_SetRelativeRotation` (`self.Cauldron`) (* (`self.CauldronEndRotation`) _cauldronrot) false false)
      (`SceneComponent.K2_SetRelativeRotation` (`self.Lever`) (`KismetMathLibrary.ComposeRotators` (`self.DefaultLeverRot`) (* (`self.InteractHandleRot`) _cauldronrot)) false false))
    (:`Finished`
      (set `self.isReady` true)
      (if (`KismetSystemLibrary.IsServer`)
        (`self.CheckForAmmoSound` 0)))))

(event `InteractableInterface.InteractableActivate`
  (params (Component :type "PrimitiveComponent Object Reference") (Instigator :type "PlayerController Object Reference") (HitIndex :type Integer) (TriggeredFromRadialWheel :type Boolean))
  (for _array_element (`self.JourneyEventTriggerOnInteract`)
    (bind _asbase_player_char_interface (cast `/Game/Systems/Interfaces/BasePlayerCharInterface` (`Controller.K2_GetPawn` Instigator)))
    (`/Game/Systems/Interfaces/BasePlayerCharInterface.AddJourneyEventInterfaceCall` _asbase_player_char_interface _array_element))
  (if (`KismetSystemLibrary.IsServer`)
    (if (== Component (`self.FireInteractBox`))
      (if (`self.isReady`)
        (set `self.Attackinstigator` Instigator)
        (bind (_hasammo_ _cauldronammoclass) (`self.CheckAmmo` true))
        (if _hasammo_
          (set `self.CauldronAmmoClass` _cauldronammoclass)
          (set `self.HasFired` true)
          (set `self.CanBeReversed` false)
          (set `self.isReady` false)
          (`self.UpdateJourneyEvent`))
        (elif (`self.CanBeReversed`)
          (set `self.HasFired` false)))
      (elif (== Component (`self.PayloadInteractBox`))
        (`InteractableInterface.InteractableActivate` (`self.BP_BAC_Storage`) null Instigator 0 false)))))

(fn `CanBePlaced`
  (params (AttachTo :type "BuildableBase Object Reference") (InstanceIndex :type Integer))
  (returns (FailedMessage :type String) (ReturnValue :type "ECanBePlacedResult Enum"))
  (locals (OverlappingActors :type "Array of Actor Object Reference"))
  (bind (_failedmessage _returnvalue) (`parent.CanBePlaced` AttachTo InstanceIndex))
  (return _failedmessage _returnvalue))

(fn `CheckAmmo`
  (params (`DeleteAmmoIfFound?` :type Boolean))
  (returns (`HasAmmo?` :type Boolean) (CauldronAmmoClass :type "/Game/Systems/Building/Placeables/SiegeDefense/BP_Cauldron_Ammo_Master Class Reference") (SoundWhileInCauldron :type "SoundCue Object Reference"))
  (locals (FoundAmmo :type Boolean))
  (bind _outrownames (`DataTableFunctionLibrary.GetDataTableRowNames` "/Game/Systems/Building/Placeables/SiegeDefense/CauldronAmmoTable.CauldronAmmoTable"))
  (for _array_element _outrownames
    (bind _returnvalue (`|GetDataTableRow` "/Game/Systems/Building/Placeables/SiegeDefense/CauldronAmmoTable.CauldronAmmoTable" _array_element)
      (:`then`
        (bind (_cauldronammoresourceid _cauldronammoclass _soundwhileincauldron) (break `/Game/Systems/Building/Placeables/SiegeDefense/CauldronAmmoTypes` _returnvalue))
        (if (>= (`ItemInventory.GetResourceCount` (`self.PlaceableInventory`) _cauldronammoresourceid false) 1)
          (set `local.FoundAmmo` true)
          (break)
          (else
            (set `local.FoundAmmo` false))))))
  (if (`local.FoundAmmo`)
    (if `DeleteAmmoIfFound?`
      (bind _returnvalue_2 (`ItemInventory.DeleteItemsByTemplate` (`self.PlaceableInventory`) _cauldronammoresourceid "consumed" 1))
      (return _returnvalue_2 _cauldronammoclass _soundwhileincauldron)
      (else
        (return true _cauldronammoclass _soundwhileincauldron)))
    (else
      (return false null null))))

(fn `OnRep_HasFired`
  (if (`self.HasFired`)
    (`self.FireSiegeEquipment`)
    (else
      (`self.ReverseSiegeEquipment`))))

(fn `OnRep_IsBoiling`
  (`self.PlayBoilingAmmoSound` (`self.IsBoiling`) (`self.BoilingSoundToPlay`)))

(fn `ProvidesShelter`
  (returns (True :type Boolean))
  (return true))

(fn `UpdateJourneyEvent`
  (bind _asbase_player_char_interface (cast `/Game/Systems/Interfaces/BasePlayerCharInterface` (`Controller.K2_GetPawn` (`self.Attackinstigator`))))
  (`/Game/Systems/Interfaces/BasePlayerCharInterface.AddJourneyEventInterfaceCall` _asbase_player_char_interface "UseSiegeCauldron"))

(fn `UserConstructionScript`
  (`parent.UserConstructionScript`)
  (set `self.DefaultLeverRot` (`SceneComponent.RelativeRotation` (`self.Lever`))))
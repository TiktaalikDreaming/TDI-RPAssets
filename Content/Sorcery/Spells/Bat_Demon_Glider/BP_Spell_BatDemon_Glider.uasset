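; Spell that summons a bat demon glider for the casting character and activates it on execution.
; The server spawns the glider when casting starts to allow replication time, destroying it if interrupted before execution.
; Clients lacking a reference search the world for the caster's unattached glider.
; Casting is blocked in dungeons, climbing-blocking volumes, shelter, or wherever a fan of forward capsule traces finds obstructed takeoff space.
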(event `self.OnSpellExecute`
  (`self.Glider`
    (:`then`
      _)
    (:`else`
      (`self.FindMyBatDemonGlider`)
      (`self.Glider`
        (:`then`
          _)
        (:`else`))))
  (bind _asbase_bpcombat (cast `/Game/Characters/BaseBPCombat` (`self.GetOwnerCharacter`)))
  (`/Game/Characters/BaseBPCombat.ClearAttackQueue` _asbase_bpcombat)
  (`/Game/Sorcery/Glider/BP_BatDemonGlider.ActivateGlider` (`self.Glider`)))

(event `self.OnStartCasting`
  (bind _character (`self.GetOwnerCharacter`))
  ;[1 1 1] Spawn the bat demon actor early so it has time to be replicated and loaded on observing clients
  (if (`KismetSystemLibrary.IsServer`)
    (bind _asbase_player_char (cast `/Game/Characters/BasePlayerChar` _character))
    (bind _returnvalue (`|SpawnActorFromClass` "/Game/Sorcery/Glider/BP_BatDemonGlider.BP_BatDemonGlider_C" (`KismetMathLibrary.Conv_VectorToTransform` (`Actor.K2_GetActorLocation` _character)) "AlwaysSpawn" "OverrideRootScale" _asbase_player_char _asbase_player_char _asbase_player_char))
    (set `self.Glider` _returnvalue)))

(event `self.OnEndCasting`
  (params (Interrupted :type Boolean))
  ;[1 1 1] In event of spellcast cancelled, clean up the bat demon actor
  (if (and Interrupted (not (`self.HasRunSpellExecute`)))
    (bind _glider (`self.Glider`)
      (:`then`
        (`Actor.K2_DestroyActor` _glider))
      (:`else`))))

(fn `CanBeCast`
  (returns (OutReason :type Text) (ReturnValue :type Boolean))
  (locals (LInsideChecker :type "/Game/Systems/Building/InsideChecker Object Reference"))
  (bind _character (`self.GetOwnerCharacter`))
  (bind (_outreason _returnvalue) (`parent.CanBeCast`))
  (if (and (== (`ConanCharacter.ClimbingBlockingVolumeCount` _character) 0) (not (`FuncomGenericLibrary.IsLocationInsideDungeon` _character (`Actor.K2_GetActorLocation` _character))))
    (bind _output_get (set `local.LInsideChecker` (`Actor.GetComponentByClass` (`self.GetOwnerCharacter`) "/Game/Systems/Building/InsideChecker.InsideChecker_C")))
    (`/Engine/EditorBlueprintResources/StandardMacros.IsValid` _output_get
      (:`Is Valid`
        (if (< (`/Game/Systems/Building/InsideChecker.InsidePercentage` (`local.LInsideChecker`)) 0.3)
          (bind _allowed (`self.CheckLineTracesForCast` :!label _label))
          (if _allowed
            (return _outreason _returnvalue)
            (else
              _))))
      (:`Is Not Valid`
        (goto _label))))
  (return "The Bat Demon cannot be summoned in a confined environment." false))

(fn `CheckLineTracesForCast`
  (returns (Allowed :type Boolean))
  (locals (ZAngleOffsets :type "Array of Float (double-precision)") (SlopeAngles :type "Array of Float (double-precision)") (LIgnoredActorsList :type "Array of Actor Object Reference"))
  (bind _character (`self.GetOwnerCharacter`))
  (bind _character_2 (`self.GetOwnerCharacter`))
  (bind _character_3 (`self.GetOwnerCharacter`))
  (bind _returnvalue (`Actor.K2_GetActorLocation` _character))
  (set `local.LIgnoredActorsList` (`Actor.GetAttachedActors` _character_3))
  (bind _actors (message `/Game/Sorcery/Spells/Casting/BPI_SpellcastFXHandler.GetRuneActors` (`Actor.GetComponentByInterface` _character_3 "/Game/Sorcery/Spells/Casting/BPI_SpellcastFXHandler.BPI_SpellcastFXHandler_C")))
  (`KismetArrayLibrary.Array_Append` (`local.LIgnoredActorsList`) _actors)
  (for _array_element (`local.ZAngleOffsets`)
    (for _array_element_2 (`local.SlopeAngles`)
      (bind _scaledcapsuleradius (`/Game/Systems/BP_MacroGlobal.GetScaledCapsuleRadius` _character_2)
        (:`Success`
          (bind _scaledcapsulehalfheight (`/Game/Systems/BP_MacroGlobal.GetScaledCapsuleHalfHeight` _character_2)
            (:`Success`
              (bind (_outhit _returnvalue_2) (`KismetSystemLibrary.CapsuleTraceSingle` (+ _returnvalue (0.0 0.0 50.0)) (+ _returnvalue (`KismetMathLibrary.TransformDirection` (`Actor.GetTransform` _character) (`KismetMathLibrary.GreaterGreater_VectorRotator` (3000.0 0.0 0.0) (`KismetMathLibrary.MakeRotator` 0.0 _array_element_2 (+ _array_element 10.0))))) _scaledcapsuleradius _scaledcapsulehalfheight "TraceTypeQuery1" false (`local.LIgnoredActorsList`) "None" true (struct :`R` 1.0 :`A` 1.0) (struct :`G` 1.0 :`A` 1.0) 10.0))
              (if _returnvalue_2
                (return false) ; If we hit something, then not allowed to take off
              )))))))
  (return true))

(fn `FindMyBatDemonGlider`
  (bind _outactors (`GameplayStatics.GetAllActorsOfClass` "/Game/Sorcery/Glider/BP_BatDemonGlider.BP_BatDemonGlider_C")) ; Due to engine limitations, we can't pass a reference to *our* Bat Demon glider within the context of this spell\nSo instead if we can't find it during spell execute, we search the world to try and find it (this only happens on clients - server already has a ref to the actor)
  (for _array_element _outactors
    (if (and (== (`/Game/Sorcery/Glider/BP_BatDemonGlider.Player` _array_element) (`self.GetOwnerCharacter`)) (not (`/Game/Sorcery/Glider/BP_BatDemonGlider.PlayerAttached` _array_element)))
      (set `self.Glider` _array_element)
      (return)))
  (return) ; Not strictly needed, but it makes the compiler happy
)
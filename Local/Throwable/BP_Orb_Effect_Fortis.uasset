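; Thrown orb ground effect that creates an oil slick, applying BP_SlipperyBuff to Conan characters inside its sphere.
; Sphere overlaps track affected characters and buff buff-capable ones on entry, while a looping server timer reapplies the buff to everyone tracked.
; Non-server instances animate a dynamic decal material with grow and roughness timelines, then fade it after a fixed delay not yet tied to the effect ending.
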(event `self.ReceiveBeginPlay`
  (`parent.ReceiveBeginPlay`)
  (if (`KismetSystemLibrary.IsServer`)
    (`KismetSystemLibrary.K2_SetTimerDelegate` (delegate `AddOilBuff`) 0.5 true)
    (else
      (`|ExecutionSequence`
        (:`then_0`
          ;[1 1 1] Grow the Decal
          (bind _returnvalue (`DecalComponent.CreateDynamicMaterialInstance` (`self.Decal`)))
          (`|ExecutionSequence`
            (:`then_0`
              (bind (_direction _grow) (`Timeline|fadein`)
                (:`Update`
                  (`MaterialInstanceDynamic.SetScalarParameterValue` _returnvalue "edgerad" (`KismetMathLibrary.Lerp` 0.0 0.5 _grow))
                  (`MaterialInstanceDynamic.SetScalarParameterValue` _returnvalue "length" (`KismetMathLibrary.Lerp` 1.0 2.0 _grow))
                  (`MaterialInstanceDynamic.SetScalarParameterValue` _returnvalue "thickness" (`KismetMathLibrary.Lerp` 100.0 3.0 _grow)))))
            (:`then_1`
              (bind (_direction_2 _roughness) (`Timeline|roughness`)
                (:`Update`
                  (`MaterialInstanceDynamic.SetScalarParameterValue` _returnvalue "roughness" _roughness))))))
        (:`then_1`
          ;[1 1 1] fade out, move to triggered by effect ending
          (`KismetSystemLibrary.Delay` 20.0)
          (bind (_direction_3 _fade) (`Timeline|fadeout` :!via `PlayFromStart`)
            (:`Update`
              (`MaterialInstanceDynamic.SetScalarParameterValue` _returnvalue "fade" _fade))))))))

(event `AddOilBuff`
  (bind _instigator (`self.Instigator`))
  (for _array_element (`self.BuffAffectedChars`)
    (message `/Game/Systems/Buffs/BuffSystemInterface.AddBuffCall` (`self.GetComponentByInterface` _array_element "/Game/Systems/Buffs/BuffSystemInterface.BuffSystemInterface_C") "/Game/Systems/Buffs/Slippery/BP_SlipperyBuff.BP_SlipperyBuff_C" _instigator 0 (`/Game/Characters/FuncomFunctionLibrary.GetControllerFromActor` _instigator))))

(event `self.Sphere.OnComponentBeginOverlap`
  (params (OverlappedComponent :type "PrimitiveComponent Object Reference") (OtherActor :type "Actor Object Reference") (OtherComp :type "PrimitiveComponent Object Reference") (OtherBodyIndex :type Integer) (bFromSweep :type Boolean) (SweepResult :type "HitResult Structure (by ref)"))
  (bind _instigator (`self.Instigator`))
  (bind _asconan_character (cast `ConanCharacter` OtherActor))
  (bind _returnvalue (`self.GetComponentByInterface` _asconan_character "/Game/Systems/Buffs/BuffSystemInterface.BuffSystemInterface_C"))
  (`/Engine/EditorBlueprintResources/StandardMacros.IsValid` _returnvalue
    (:`Is Valid`
      (`KismetArrayLibrary.Array_Add` (`self.BuffAffectedChars`) _asconan_character)
      (message `/Game/Systems/Buffs/BuffSystemInterface.AddBuffCall` _returnvalue "/Game/Systems/Buffs/Slippery/BP_SlipperyBuff.BP_SlipperyBuff_C" _instigator 0 (`/Game/Characters/FuncomFunctionLibrary.GetControllerFromActor` _instigator)))))

(event `self.Sphere.OnComponentEndOverlap`
  (params (OverlappedComponent :type "PrimitiveComponent Object Reference") (OtherActor :type "Actor Object Reference") (OtherComp :type "PrimitiveComponent Object Reference") (OtherBodyIndex :type Integer))
  (bind _asconan_character (cast `ConanCharacter` OtherActor))
  (`KismetArrayLibrary.Array_RemoveItem` (`self.BuffAffectedChars`) _asconan_character))

(fn `UserConstructionScript`
  (`parent.UserConstructionScript`))
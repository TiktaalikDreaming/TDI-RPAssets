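; Nitric alchemist crafting workstation placeable, apparently set up for a chance to blow up when crafting.
; On BeginPlay it listens for the crafting queue's item-started signal, then compares a fixed zero roll against Chancetoblow, but neither outcome triggers anything yet.
; It also exposes the artisan thrall inventory and reports impact radius, strength, player-damage status and the owner as attacker.
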(event `self.ReceiveBeginPlay`
  (`parent.ReceiveBeginPlay`)
  (add `CraftingQueue.SignalItemStartedCrafting` (`self.CraftingQueue`) (delegate `SignalItemStartedCrafting_Event_1`)))

(event `SignalItemStartedCrafting_Event_1`
  (params (recipeItem :type "RecipeItem Object Reference") (craftingCharacterUID :type "UniqueID Object Reference"))
  (if (< (`KismetMathLibrary.RandomFloatInRange` 0.0) (`self.Chancetoblow`))
    _))

(fn `Get Attacker Unique ID`
  (returns (`Return Value` :type "UniqueID Object Reference"))
  (return (`self.OwnerUniqueID`)))

(fn `Get Impact Radius`
  (returns (`Impact Radius` :type "Float (double-precision)"))
  (return 7500.0))

(fn `Get Impact Strength`
  (returns (`Impact Strength` :type "Float (double-precision)"))
  (return 3.0))

(fn `GetArtisanThrallInventory`
  (returns (ReturnValue :type "ItemInventory Object Reference"))
  (return (`self.ThrallInventory`)))

(fn `Is Player Damage`
  (returns (`Return Value` :type Boolean))
  (return true))

(fn `UserConstructionScript`
  (`parent.UserConstructionScript`))
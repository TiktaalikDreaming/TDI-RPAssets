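; Thrown offhand cake projectile that spins in flight, extending a parent projectile Blueprint.
; On begin play it applies the launch rotation to the swivel and tracer particles, then Tick spins the swivel from accumulated fly time, skipped on dedicated servers.
; Stopping destroys the spinning disc particle.
; Spawning the dummy projectile first resets mesh scale so the resulting pickable looks correct, then defers to the parent.
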(event `self.ReceiveBeginPlay`
  (`parent.ReceiveBeginPlay`)
  (`SceneComponent.K2_AddRelativeRotation` (`self.ProjectileSwivel`) (`self.ProjectileLaunchRotation`) false false)
  (`SceneComponent.K2_SetRelativeRotation` (`self.TracerParticleSystem`) (`self.ProjectileLaunchRotation`) false false))

(event `self.ReceiveTick`
  (params (DeltaSeconds :type "Float (single-precision)"))
  (if (not (`KismetSystemLibrary.IsDedicatedServer`))
    (bind _output_get (set `self.local ProjectileTotalFlyTime` (+ (`self.local ProjectileTotalFlyTime`) (* DeltaSeconds -1.0))))
    (`SceneComponent.K2_SetRelativeRotation` (`self.ProjectileSwivel`) (`KismetMathLibrary.ComposeRotators` (* (`self.ProjectileRotateSpeed`) _output_get) (`self.ProjectileLaunchRotation`)) false false)))

(event `self.StopProjectile`
  (`parent.StopProjectile`)
  (`ActorComponent.K2_DestroyComponent` (`self.SpinningDiscParticle`)))

(event `self.SpawnDummyProjectile`
  (params (HitResultFromProjectile :type "HitResult Structure") (ProjectileDummyLifetime :type "Float (single-precision)") (IsLootable :type Boolean) (ShouldBreakOnImpact :type Boolean))
  ;[1 1 1] Undo projectile scale so the pickable doesnt look silly
  (`SceneComponent.SetRelativeScale3D` (`self.ProjectileMesh`) (1.0 1.0 1.0))
  (`parent.SpawnDummyProjectile` HitResultFromProjectile ProjectileDummyLifetime IsLootable ShouldBreakOnImpact))

(fn `UserConstructionScript`
  (`parent.UserConstructionScript`))
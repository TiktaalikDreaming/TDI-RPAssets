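; A placeable thrall feeding container whose food plane visually reflects how full its inventory is.
; On begin play and on item add or remove, the fill ratio sets the plane's height and scrubs a timeline curve that scales it to fit the bowl, hiding it when empty.
; Non-dedicated instances create an inventory client monitor so contents load without interaction.
; It also exposes its ThrallItemDistributor through a getter.
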(event `self.ReceiveBeginPlay`
  (bind _placeableinventory (`self.PlaceableInventory`))
  (bind _returnvalue (/ (`KismetMathLibrary.Conv_IntToDouble` (`ItemInventory.GetPopulatedItemCount` (`self.PlaceableInventory`) 0 -1)) (`KismetMathLibrary.Conv_IntToDouble` (`ItemInventory.MaxItemCount` (`self.PlaceableInventory`)))))
  (`parent.ReceiveBeginPlay`)
  (if (`KismetSystemLibrary.IsDedicatedServer`)
    _
    (else
      _))
  (`|ExecutionSequence`
    (:`then_0`
      ;[0.02499 0.09524 0.16] Make sure the the inventory is loaded even if it hasn't been interacted with.
      (if (not (`KismetSystemLibrary.IsDedicatedServer`))
        (bind _returnvalue_2 (`|GenericCreateObject` "/Script/ConanSandbox.ItemInventoryClientMonitor" self))
        (`ItemInventoryClientMonitor.SetInventory` _returnvalue_2 (`self.PlaceableInventory`))))
    (:`then_1`
      (add `ItemInventory.SignalItemAdded` _placeableinventory (delegate `SetFoodPlaneHeight`))
      (add `ItemInventory.SignalItemRemoved` _placeableinventory (delegate `SetFoodPlaneHeight`)))
    (:`then_2`
      ;[1 0.6413 0.1882] Set Z location of FoodPlane
      (`SceneComponent.K2_SetRelativeLocation` (`self.FoodPlane`) (`KismetMathLibrary.MakeVector` 0.0 0.0 (`KismetMathLibrary.Lerp` -40.0 0.0 _returnvalue)) false false :!label _label)
      ;[1 0.6413 0.1882] Set XY scale based on curve to fit the bowl.
      (bind (_direction _scale) (`Timeline|Timeline_0` :`NewTime` _returnvalue :!via `SetNewTime`)
        (:`Update`
          (`SceneComponent.SetRelativeScale3D` (`self.FoodPlane`) (`KismetMathLibrary.MakeVector` _scale _scale 1.0))
          ;[1 0.6413 0.1882] Handle Visibility
          (if (== (`ItemInventory.GetPopulatedItemCount` (`self.PlaceableInventory`) 0 -1) 0)
            (`SceneComponent.SetVisibility` (`self.FoodPlane`) false false)
            (else
              (`SceneComponent.SetVisibility` (`self.FoodPlane`) true false))))))))

(event `SetFoodPlaneHeight`
  (params (index :type Integer) (item :type "GameItem Object Reference") (dstInventory :type "ItemInventory Object Reference") (dstIndex :type Integer))
  ;[1 0.6413 0.1882] Set Z location of FoodPlane
  (goto _label))

(fn `GetItemDistributor`
  (returns (ItemDistributor :type "/Game/Systems/Building/Placeables/ItemDistributor Object Reference"))
  (return (`self.ThrallItemDistributor`)))

(fn `UserConstructionScript`
  (`parent.UserConstructionScript`))
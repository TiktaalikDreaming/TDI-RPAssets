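; BP_AC_Buff_PostHigh is a buff component for a post-high penalty that lowers the owning character's maximum stamina while active.
; Start and clear effects apply opposite merged StaminaMax modifiers, so the penalty reverses when the buff ends.
; On start it caches the owner's BP_HungerSystem, then each tick drains current food by a WaterMultiplier fraction.
; The effect description reports increased thirst, although the tick changes only food.
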(event `self.GameplayEffectToApplyOnBuffStart`
  (`ConanCharacter.AddIntStatModifier` (`self.OwningCharacter`) "StaminaMax" "Buff" "Add" (* (`self.MaxStaminaPenalty`) -1) "Merge"))

(event `self.GameplayEffectToApplyOnBuffCleared`
  (`ConanCharacter.AddIntStatModifier` (`self.OwningCharacter`) "StaminaMax" "Buff" "Add" (`self.MaxStaminaPenalty`) "Merge"))

(event `self.StartBuff`
  (params (BuffPotency :type Integer) (OwningCharacter :type "ConanCharacter Object Reference") (Instigator :type "Controller Object Reference"))
  (bind _returnvalue (`Actor.GetComponentByClass` (`self.OwningCharacter`) "/Game/Systems/Hunger/BP_HungerSystem.BP_HungerSystem_C"))
  (`parent.StartBuff` BuffPotency OwningCharacter Instigator)
  (`/Engine/EditorBlueprintResources/StandardMacros.IsValid` _returnvalue
    (:`Is Valid`
      (set `self.HungerSystem` _returnvalue))))

(event `self.GameplayEffectToApplyOnBuffTick`
  (bind _hungersystem (`self.HungerSystem`))
  (`/Engine/EditorBlueprintResources/StandardMacros.IsValid` _hungersystem
    (:`Is Valid`
      (bind _value (`/Game/Systems/Hunger/BP_HungerSystem.GetFoodCurrent` _hungersystem))
      (`/Game/Systems/Hunger/BP_HungerSystem.SetFoodCurrent` _hungersystem _value (- _value (* _value (`self.WaterMultiplier`)))))))

(fn `GetEffectDescription`
  (returns (Description :type Text))
  (return (`|FormatText` "Maximum Stamina reduced  by {StaminaMaxReduction}. Thirst rate slightly increased." (`self.MaxStaminaPenalty`))))
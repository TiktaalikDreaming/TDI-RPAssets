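; Explosive trap Blueprint that plays its detonation effects and reports its damage as player damage attributed to the owner's unique ID.
; On activation, outside dedicated servers, it stops the fuse sound and dud smoke, then plays the trigger sound, explosion effect and epicentre-oriented camera shake, and hides the mesh.
; The explosion effects run only when the dud smoke component is valid.
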(event `/Game/Systems/Building/Placeables/BP_PL_Trap.Play Trap Activate Effects`
  (bind _staticmesh (`self.StaticMesh`))
  (bind _returnvalue (`SceneComponent.K2_GetComponentLocation` _staticmesh))
  ;[1 0.6413 0.1882] Effects
  (if (not (`KismetSystemLibrary.IsDedicatedServer`))
    ;;[0.02499 0.09524 0.16] Disable dud effects.
    (bind _fusesound (`self.FuseSound`)
      (:`then`
        (`ConanAudioComponent.Stop` _fusesound))
      (:`else`
        _))
    (bind _fusedudsmoke (`self.FuseDudSmoke`)
      (:`then`
        (`ActorComponent.Deactivate` _fusedudsmoke)
        ;;[0 0.605 0.605] Play Explosion Sound
        (`GameplayStatics.PlaySoundAtLocation` (`self.S_Trigger_Activate`) _returnvalue)
        (`ActorComponent.Activate` (`self.Explosion`) false)
        (`GameplayStatics.PlayWorldCameraShake` "/Game/Items/Explosives/CameraShake_Explosion.CameraShake_Explosion_C" _returnvalue 0.0 102404096.0 1.0 true)
        (`SceneComponent.SetVisibility` _staticmesh false false))
      (:`else`))))

(fn `GetAttackerUniqueID`
  (returns (ReturnValue :type "UniqueID Object Reference"))
  (return (`self.OwnerUniqueID`)))

(fn `IsPlayerDamage`
  (returns (ReturnValue :type Boolean))
  (return true))

(fn `IsThrallDamage`
  (returns (ReturnValue :type Boolean))
  (return false))

(fn `UserConstructionScript`
  (`parent.UserConstructionScript`))
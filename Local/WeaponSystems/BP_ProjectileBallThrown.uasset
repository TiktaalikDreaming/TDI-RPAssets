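; Thrown projectile ball weapon item that is used up from its stack as it is thrown.
; On throw it hides the visual actor and decrements the stack, except for non-thrall NPCs, who throw without consuming.
; When the stack runs out, the server force-unequips it for players or removes it from other characters' inventories.
; Attack end shows the visual again, and the launcher template ID comes from the weapon itself.
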(fn `GetLauncherTemplateId`
  (params (Projectile :type "/Game/Items/Weapons/BP_BaseProjectile Object Reference") (Weapon :type "/Game/Items/BPGameItemWeapon Object Reference"))
  (returns (PickableAmmoTemplateId :type Integer))
  (return (`GameItem.TemplateID` Weapon)))

(fn `WeaponAttackEnd`
  (returns (Success :type Boolean))
  (`Actor.SetActorHiddenInGame` (`self.VisualActor`) false)
  (return true))

(fn `WeaponThrown`
  (returns (Success :type Boolean))
  (bind _returnvalue (`self.GetOwnerInventory`))
  (bind _returnvalue_2 (`self.GetIntStat` "StackSize"))
  (`Actor.SetActorHiddenInGame` (`self.VisualActor`) true)
  (bind _asconan_character (cast `ConanCharacter` (`self.GetOwner`))
    (:`then`
      (if (`ConanCharacter.IsNonThrallNPC` _asconan_character)
        (return true)
        (else
          _)))
    (:`CastFailed`
      _))
  (if (< _returnvalue_2 2)
    (`self.SetStackSize` -1 "consumed")
    (else
      (`self.SetStackSize` (- _returnvalue_2 1) "consumed")))
  (`/Game/Systems/BP_MacroGlobal.And+Branch` (< (`self.GetIntStat` "StackSize") 1) (`KismetSystemLibrary.IsServer`)
    (:`True`
      (bind _asconan_character_2 (cast `ConanCharacter` (`self.GetOwner`))
        (:`then`
          (if (`ConanCharacter.IsPlayer` _asconan_character_2)
            (`self.ForceUnequip`)
            (else
              (`ItemInventory.RemoveItem` _returnvalue (`ItemInventory.GetItemIndex` _returnvalue self) "consumed" null)))
          (return true))
        (:`CastFailed`
          _)))
    (:`False`
      _))
  (return true))
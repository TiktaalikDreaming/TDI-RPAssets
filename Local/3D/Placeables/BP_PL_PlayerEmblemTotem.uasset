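; Placeable clan emblem totem that only guild members can place and that displays the owning guild's emblem on its mesh.
; Interaction checks membership, rank and single-user occupancy via the game state, then grants emblem feats and opens GuildEmblemView with a temporary material.
; Cancelling on the server applies the emblem material and releases occupancy.
; BeginPlay applies the emblem, waiting on owner-ID or data-loaded signals when needed, and syncs emblem data.
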(event `InteractableInterface.InteractableActivate`
  (params (Component :type "PrimitiveComponent Object Reference") (Instigator :type "PlayerController Object Reference") (HitIndex :type Integer) (TriggeredFromRadialWheel :type Boolean))
  (bind _returnvalue (`Controller.K2_GetPawn` Instigator))
  (`parent.InteractableActivate` Component Instigator HitIndex TriggeredFromRadialWheel)
  (if (`Controller.IsLocalController` (`GameplayStatics.GetPlayerController` 0))
    (bind _returnvalue_2 (`GUIModuleController.GetModule` (`GUIModuleController.GetGUIModuleController`) "GuildEmblemView"))
    (add `GUIModule.SignalActivated` _returnvalue_2 (delegate `OnGuildEmblemViewActive`)))
  (bind _asconan_character (cast `ConanCharacter` _returnvalue))
  (if (== (`ConanCharacter.GetGuildId` _asconan_character) (`self.OwnerUniqueID`))
    (bind _uniqueid (message `/Game/Systems/Interfaces/BasePlayerCharInterface.GetUniqueID` _asconan_character))
    (bind _returnvalue_3 (`ConanCharacter.GetGuild` _asconan_character))
    (if (`KismetSystemLibrary.IsValid` _returnvalue_3)
      (bind _returnvalue_4 (`Guild.GetGuildEmblemRankRestriction` self (`Guild.GetId` _returnvalue_3)))
      (if (>= (`Guild.GetPlayerRank` _returnvalue_3 _uniqueid) _returnvalue_4)
        (bind _asconan_game_state (cast `ConanGameState` (`GameplayStatics.GetGameState`)))
        (bind _asconan_player_controller (cast `ConanPlayerController` Instigator))
        (bind _returnvalue_5 (`ConanGameState.RequestGuildEmblemPlaceableOccupy` _asconan_game_state _asconan_player_controller))
        (if (!= _returnvalue_5 _asconan_player_controller)
          (`ConanCharacter.ClientHUDShowFIFOEmblem` _asconan_character "EmblemOccupied" (`self.OccupiedMessage`))
          (else
            (bind _returnvalue_6 (`ConanCharacter.GetProgressionSystem` _asconan_character))
            (`self.GrantFeats` _returnvalue_6 :!pinned true) ; Grant Feats
            (`ConanCharacter.SetInteractingActor` _asconan_character self "GuildEmblemView")
            (bind _asbase_bpchar (cast `/Game/Characters/BaseBPChar` _returnvalue))
            (`/Game/Characters/BaseBPChar.SetEmblemPlaceableTempMaterial` _asbase_bpchar self (`self.EmblemMaterialIndex`))
            (set `self.InteractingCharacter` _asconan_character)))
        (else
          (`ConanCharacter.ClientHUDShowFIFOEmblem` _asconan_character "EmblemRankRestriction" (`self.RankRestrictionMessage`)))))
    (else
      (`ConanCharacter.ClientHUDShowFIFOEmblem` _asconan_character "EmblemNotMemberOfClan" (`self.NotMemberMessage`)))))

(event `self.OnPlaced`
  (params (PlacedBy :type "ConanCharacter Object Reference"))
  (`parent.OnPlaced` PlacedBy)
  (bind _asconan_game_state (cast `ConanGameState` (`GameplayStatics.GetGameState`)))
  (`ConanGameState.ServerClanEmblemTotemPlaced` _asconan_game_state (`ConanCharacter.GetGuildId` PlacedBy)))

(event `InteractableInterface.ClientInteractableActivate`
  (params (Component :type "PrimitiveComponent Object Reference") (Instigator :type "PlayerController Object Reference") (HitIndex :type Integer))
  (`parent.ClientInteractableActivate` Component Instigator HitIndex)
  (bind _returnvalue (`GUIModuleController.GetModule` (`GUIModuleController.GetGUIModuleController`) "GuildEmblemView"))
  (add `GUIModule.SignalActivated` _returnvalue (delegate `OnGuildEmblemViewActive`)))

(event `OnGuildEmblemViewActive`
  (params (module :type "GUIModule Object Reference") (isActive :type Boolean))
  (if isActive
    (`PrimitiveComponent.SetCollisionResponseToChannel` (`self.StaticMesh`) "ECC_GameTraceChannel16" "ECR_Ignore")
    (else
      (`PrimitiveComponent.SetCollisionResponseToChannel` (`self.StaticMesh`) "ECC_GameTraceChannel16" "ECR_Overlap"))))

(event `self.ReceiveBeginPlay`
  (bind _owneruniqueid (`self.OwnerUniqueID`))
  (`parent.ReceiveBeginPlay`)
  (if (`KismetSystemLibrary.IsServer`)
    (bind _asconan_game_state (cast `ConanGameState` (`GameplayStatics.GetGameState`) :!label _label))
    (bind _returnvalue (`Guild.GetGuildEmblem` self _owneruniqueid))
    (if (`KismetSystemLibrary.IsValid` _returnvalue)
      (`PrimitiveComponent.SetMaterial` (`self.StaticMesh`) (`self.EmblemMaterialIndex`) _returnvalue)
      (else
        (add `ConanGameState.SignalOnGuildEmblemDataLoaded` _asconan_game_state (delegate `OnGuildEmblemDataLoaded`))))
    (bind _asconan_character (cast `ConanCharacter` (`GameplayStatics.GetPlayerCharacter` 0) :!label _label_2)
      (:`then`
        (bind _returnvalue_2 (`ConanCharacter.GetProgressionSystem` _asconan_character))
        (`self.GrantFeats` _returnvalue_2 :!pinned true) ; Grant Feats
        (`ConanCharacter.ServerSyncClanEmblemDataWithClient` _asconan_character _owneruniqueid))
      (:`CastFailed`
        (bind _asconan_player_controller (cast `ConanPlayerController` (`GameplayStatics.GetPlayerController` 0)))
        (add `ConanPlayerController.SignalCharacterReadyClient` _asconan_player_controller (delegate `CharacterReady`))))
    (else
      (add `self.SignalReceivedOwnerUniqueID` (delegate `OnReceivedOwnerUniqueID`)))))

(event `OnReceivedOwnerUniqueID`
  (goto _label))

(event `CharacterReady`
  (goto _label_2))

(event `OnGuildEmblemDataLoaded`
  (params (GuildId :type "UniqueID Object Reference"))
  (if (== GuildId (`self.OwnerUniqueID`))
    (bind _returnvalue (`Guild.GetGuildEmblem` self GuildId))
    (`PrimitiveComponent.SetMaterial` (`self.StaticMesh`) (`self.EmblemMaterialIndex`) _returnvalue)))

(event `InteractableInterface.InteractableOnCancel`
  (params (Instigator :type "PlayerController Object Reference"))
  (bind _returnvalue (`Controller.K2_GetPawn` Instigator))
  (`parent.InteractableOnCancel` Instigator)
  (set `self.InteractingCharacter` null)
  (bind _asconan_character (cast `ConanCharacter` _returnvalue))
  (bind _returnvalue_2 (`ConanCharacter.GetInteractingActor` _asconan_character))
  (if (and (`KismetSystemLibrary.IsValid` _returnvalue_2) (`KismetSystemLibrary.IsServer`))
    (bind _asbase_bpchar (cast `/Game/Characters/BaseBPChar` _returnvalue))
    (`/Game/Characters/BaseBPChar.SetEmblemPlaceableMaterial` _asbase_bpchar self (`self.EmblemMaterialIndex`))
    (bind _asconan_game_state (cast `ConanGameState` (`GameplayStatics.GetGameState`)))
    (bind _asconan_player_controller (cast `ConanPlayerController` Instigator))
    (`ConanGameState.EndGuildEmblemPlaceableOccupy` _asconan_game_state _asconan_player_controller)))

(fn `CanBePlaced`
  (params (AttachTo :type "BuildableBase Object Reference") (InstanceIndex :type Integer))
  (returns (FailedMessage :type String) (ReturnValue :type "ECanBePlacedResult Enum"))
  (bind (_failedmessage _returnvalue) (`parent.CanBePlaced` AttachTo InstanceIndex))
  (if (`|EnumEquality` _returnvalue "Success")
    (if (`KismetSystemLibrary.IsServer`)
      (bind _asconan_game_state (cast `ConanGameState` (`GameplayStatics.GetGameState`))
        (:`then`
          (bind _returnvalue_2 (`ConanGameState.GetServerGuildFromId` _asconan_game_state (`self.OwnerUniqueID`)))
          (if (`KismetSystemLibrary.IsValid` _returnvalue_2)
            (return "" "Success")
            (else
              _)))
        (:`CastFailed`
          _))
      (else
        (bind _asconan_player_controller (cast `ConanPlayerController` (`GameplayStatics.GetPlayerController` 0))
          (:`then`
            (if (`KismetSystemLibrary.IsValid` (`ConanCharacter.GetGuild` (`ConanPlayerController.GetConanCharacter` _asconan_player_controller)))
              (return "" "Success")
              (else
                _)))
          (:`CastFailed`
            _))))
    (return (`KismetTextLibrary.Conv_TextToString` (`self.CannotPlaceMessage`)) "Fail_NotMemberOfClan")
    (else
      (return _failedmessage _returnvalue))))

(fn `GrantFeats`
  (params (ProgressionSystem :type "ProgressionSystem Object Reference"))
  (`|ExecutionSequence`
    (:`then_0`
      (`ProgressionSystem.ServerForceLearnFeat` ProgressionSystem 96151 true false) ; BaseGame
      (`ProgressionSystem.ServerForceLearnFeat` ProgressionSystem 96152 true false)
      (`ProgressionSystem.ServerForceLearnFeat` ProgressionSystem 96153 true false)
      (`ProgressionSystem.ServerForceLearnFeat` ProgressionSystem 96154 true false)
      (`ProgressionSystem.ServerForceLearnFeat` ProgressionSystem 96155 true false)
      (`ProgressionSystem.ServerForceLearnFeat` ProgressionSystem 96156 true false)
      (`ProgressionSystem.ServerForceLearnFeat` ProgressionSystem 96157 true false)
      (`ProgressionSystem.ServerForceLearnFeat` ProgressionSystem 96158 true false)
      (`ProgressionSystem.ServerForceLearnFeat` ProgressionSystem 96159 true false)
      (`ProgressionSystem.ServerForceLearnFeat` ProgressionSystem 96160 true false))
    (:`then_1`
      (`ProgressionSystem.ServerForceLearnFeat` ProgressionSystem 96161 true false) ; DLC Special
      (`ProgressionSystem.ServerForceLearnFeat` ProgressionSystem 96162 true false)
      (`ProgressionSystem.ServerForceLearnFeat` ProgressionSystem 96163 true false)
      (`ProgressionSystem.ServerForceLearnFeat` ProgressionSystem 96164 true false)
      (`ProgressionSystem.ServerForceLearnFeat` ProgressionSystem 96165 true false)
      (`ProgressionSystem.ServerForceLearnFeat` ProgressionSystem 96166 true false)
      (`ProgressionSystem.ServerForceLearnFeat` ProgressionSystem 96167 true false)
      (`ProgressionSystem.ServerForceLearnFeat` ProgressionSystem 96168 true false)
      (`ProgressionSystem.ServerForceLearnFeat` ProgressionSystem 96169 true false)
      (`ProgressionSystem.ServerForceLearnFeat` ProgressionSystem 96170 true false)
      (`ProgressionSystem.ServerForceLearnFeat` ProgressionSystem 96171 true false)
      (`ProgressionSystem.ServerForceLearnFeat` ProgressionSystem 96172 true false))))

(fn `InteractableActivateDisabled`
  (params (InteractingCharacter :type "ConanCharacter Object Reference"))
  (returns (ReturnValue :type Boolean))
  (bind _returnvalue (`parent.InteractableActivateDisabled` InteractingCharacter))
  (return _returnvalue))

(fn `UserConstructionScript`
  (`parent.UserConstructionScript`))
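; Crafting station dryer placeable that swaps its mesh to show whether it holds certain items, apparently meats.
; Inventory add and remove signals flip the UpdateVisuals bool, used purely as a RepNotify trigger to refresh visuals.
; The refresh checks the inventory against hardcoded template IDs and picks the filled or empty wicker dryer mesh.
; The artisan thrall inventory getter is left empty.
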(event `self.PlaceableInventory.SignalItemAdded`
  (params (index :type Integer) (item :type "GameItem Object Reference") (srcInventory :type "ItemInventory Object Reference") (srcIndex :type Integer))
  (set `self.UpdateVisuals` (not (`self.UpdateVisuals`)) :!label _label))

(event `self.PlaceableInventory.SignalItemRemoved`
  (params (index :type Integer) (item :type "GameItem Object Reference") (dstInventory :type "ItemInventory Object Reference") (dstIndex :type Integer))
  (goto _label))

(event `UpdateVisualMeats`
  (bind _placeableinventory (`self.PlaceableInventory`))
  (if (or (`ItemInventory.HasItemByTemplateID` _placeableinventory 13001 1) (`ItemInventory.HasItemByTemplateID` _placeableinventory 13002 1) (`ItemInventory.HasItemByTemplateID` _placeableinventory 13003 1) (`ItemInventory.HasItemByTemplateID` _placeableinventory 18010 1) (`ItemInventory.HasItemByTemplateID` _placeableinventory 18011 1) (`ItemInventory.HasItemByTemplateID` _placeableinventory 18012 1) (`ItemInventory.HasItemByTemplateID` _placeableinventory 18013 1) (`ItemInventory.HasItemByTemplateID` _placeableinventory 18014 1) (`ItemInventory.HasItemByTemplateID` _placeableinventory 18020 1) (`ItemInventory.HasItemByTemplateID` _placeableinventory 18021 1) (`ItemInventory.HasItemByTemplateID` _placeableinventory 18022 1))
    (`StaticMeshComponent.SetStaticMesh` (`self.StaticMesh`) "/Game/Mods/TDIRPAssets/3D/Placeables/Benches/Replacers/SM_WhickerDryer_on.SM_WhickerDryer_on")
    (else
      (`StaticMeshComponent.SetStaticMesh` (`self.StaticMesh`) "/Game/Mods/TDIRPAssets/3D/Placeables/Benches/Replacers/SM_WhickerDryer.SM_WhickerDryer"))))

(fn `GetArtisanThrallInventory`
  (returns (ReturnValue :type "ItemInventory Object Reference"))
  (return null))

(fn `OnRep_UpdateVisuals`
  (`self.UpdateVisualMeats`))

(fn `UserConstructionScript`
  (`parent.UserConstructionScript`))
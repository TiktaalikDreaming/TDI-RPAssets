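; Tan pot crafting station placeable that supports artisan thralls, exposing its thrall inventory to the station logic.
; Outside brush mode, it binds to the tanner work slot's state changes on BeginPlay, applies the current state immediately, and unbinds on EndPlay.
; Props are hidden while the slot is in use and shown when it is deactivated, available or reserved.
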(event `self.ReceiveBeginPlay`
  (`parent.ReceiveBeginPlay`)
  (if (not (`self.IsABrush`))
    (add `SmartObjectSlotComponent.OnStateChanged` (`self.SOS_Work_Tanner`) (delegate `SlotStateChanged`))
    (`self.SlotStateChanged` null "Deactivated" (`SmartObjectSlotComponent.GetState` (`self.SOS_Work_Tanner`)))))

(event `SlotStateChanged`
  (params (SlotComponent :type "SmartObjectSlotComponent Object Reference") (PrevState :type "ESmartObjectSlotState Enum") (NewState :type "ESmartObjectSlotState Enum"))
  (switch `ESmartObjectSlotState` NewState
    (:`Deactivated`
      (`self.TogglePropVisibility` true :!label _label))
    (:`Available`
      (goto _label))
    (:`Reserved`
      (goto _label))
    (:`InUse`
      (`self.TogglePropVisibility` false))))

(event `self.ReceiveEndPlay`
  (params (EndPlayReason :type "EEndPlayReason Enum" :default "Destroyed"))
  (`parent.ReceiveEndPlay` EndPlayReason)
  (clear `SmartObjectSlotComponent.OnStateChanged` (`self.SOS_Work_Tanner`)))

(fn `CanStationUseThralls`
  (returns (ReturnValue :type Boolean))
  (return true))

(fn `GetArtisanThrallInventory`
  (returns (ReturnValue :type "ItemInventory Object Reference"))
  (return (`self.ThrallInventory`)))

(fn `UserConstructionScript`
  (`parent.UserConstructionScript`))
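; BP_PL_CraftingStation_AllCraft is a placeable crafting bench Blueprint that supports artisan thralls.
; It always reports that it can use thralls and exposes ThrallInventory as its artisan thrall inventory.
; On BeginPlay it switches all lights off through BPBACTurnLightOnOff if the crafting queue is already running, then calls the parent logic.
; The construction script only defers to the parent, and the IsABrush check and EndPlay do nothing.
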(event `self.ReceiveBeginPlay`
  (if (`CraftingQueue.IsRunning` (`self.CraftingQueue`))
    (`/Game/Systems/Building/BuildingActorComponents/BP_BAC_TurnLightOnOff.TurnOffAll` (`self.BP_BAC_TurnLightOnOff`)))
  (`parent.ReceiveBeginPlay`)
  (if (`self.IsABrush`)
    _))

(event `self.ReceiveEndPlay`
  (params (EndPlayReason :type "EEndPlayReason Enum" :default "Destroyed")))

(fn `CanStationUseThralls`
  (returns (ReturnValue :type Boolean))
  (return true))

(fn `GetArtisanThrallInventory`
  (returns (ReturnValue :type "ItemInventory Object Reference"))
  (return (`self.ThrallInventory`)))

(fn `UserConstructionScript`
  (`parent.UserConstructionScript`))
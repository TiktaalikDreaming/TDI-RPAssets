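; BP_PL_WorkStation_DyeingBucket is a placeable dyeing-bucket crafting station that can use thralls.
; It is a thin child Blueprint that overrides getters to expose its dye item inventory and artisan thrall inventory.
; It also names DyeingStationInventory as the center panel of the crafting GUI.
; The event graph is inactive and the construction script only calls the parent.
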(fn `CanStationUseThralls`
  (returns (ReturnValue :type Boolean))
  (return true))

(fn `ClientGetCraftingGUICenterPanel`
  (params (Instigator :type "PlayerController Object Reference"))
  (returns (ReturnValue :type Name))
  (return "DyeingStationInventory"))

(fn `GetArtisanThrallInventory`
  (returns (ReturnValue :type "ItemInventory Object Reference"))
  (return (`self.ThrallInventory`)))

(fn `GetDyeItemInventory`
  (returns (ReturnValue :type "ItemInventory Object Reference"))
  (return (`self.DyeInventory`)))

(fn `UserConstructionScript`
  (`parent.UserConstructionScript`))
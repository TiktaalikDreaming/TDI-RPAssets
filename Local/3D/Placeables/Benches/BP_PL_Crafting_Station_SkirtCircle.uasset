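; Placeable SkirtCircle crafting station with portal, portal-interrupt and corpse-summon effects.
; Events start the effects, switching portal and corpse FX off after a fixed delay as a stopgap, while interruption swaps portal FX immediately.
; Interaction overrides defer to the parent only while Interactable is set, otherwise blocking loot, menu and UI module.
; FindPositionOutsideCircle projects a player to DesiredOffset from the lowered crafting center, returning that center as look-at target.
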(event `PlayFX_Portal`
  (`ActorComponent.Activate` (`self.FX_Portal`) true)
  (`KismetSystemLibrary.Delay` 12.0)
  ;[1 0 0] this should be disabled once the FX are set to stop on their own
  (`ActorComponent.Deactivate` (`self.FX_Portal`)))

(event `PlayFX_SummonCorpse`
  (`ActorComponent.Activate` (`self.FX_RecallCorpse`) true)
  (`KismetSystemLibrary.Delay` 12.0)
  ;[1 0 0] this should be disabled once the FX are set to stop on their own
  (`ActorComponent.Deactivate` (`self.FX_RecallCorpse`)))

(event `PlayFX_PortalInterrupt`
  (`ActorComponent.Deactivate` (`self.FX_Portal`))
  (`ActorComponent.Activate` (`self.FX_Portal_Interrupt`) true))

(fn `FindPositionOutsideCircle`
  (params (PlayerToMove :type "Actor Object Reference"))
  (returns (Position :type "Vector Structure") (LookAt :type "Vector Structure"))
  (locals (PlayerPosition :type "Vector Structure") (DesiredOffset :type "Float (double-precision)" :default 450.0) (CenterPosition :type "Vector Structure" :default (0.0 0.0 0.0)))
  (bind (_returnvalue_x _returnvalue_y) (`KismetMathLibrary.BreakVector` (`self.K2_GetActorLocation` PlayerToMove)))
  (bind _output_get (set `local.CenterPosition` (- (`SceneComponent.K2_GetComponentLocation` (`self.CraftingLocation`)) (0.0 0.0 40.0))))
  (set `local.PlayerPosition` (`KismetMathLibrary.MakeVector` _returnvalue_x _returnvalue_y (.z _output_get)))
  (return (`KismetMathLibrary.VLerp` (`local.CenterPosition`) (`local.PlayerPosition`) (/ (`local.DesiredOffset`) (`KismetMathLibrary.VSize` (- (`local.CenterPosition`) (`local.PlayerPosition`))))) (`local.CenterPosition`)))

(fn `InteractableCanBeLooted`
  (params (InteractingCharacter :type "ConanCharacter Object Reference"))
  (returns (ReturnValue :type Boolean))
  (bind _returnvalue (`parent.InteractableCanBeLooted` InteractingCharacter))
  (if (`self.Interactable`)
    (return _returnvalue)
    (else
      (return false))))

(fn `InteractableGetUIModuleName`
  (returns (ReturnValue :type Name))
  (bind _returnvalue (`parent.InteractableGetUIModuleName`))
  (if (`self.Interactable`)
    (return _returnvalue)
    (else
      (return "None"))))

(fn `InteractableMenuDisabled`
  (params (InteractingCharacter :type "ConanCharacter Object Reference"))
  (returns (ReturnValue :type Boolean))
  (bind _returnvalue (`parent.InteractableMenuDisabled` InteractingCharacter))
  (if (`self.Interactable`)
    (return _returnvalue)
    (else
      (return true))))

(fn `UserConstructionScript`
  (`parent.UserConstructionScript`))
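; Placeable signpost actor that opens a long-text input popup when a player interacts with it.
; CustomInteraction sets the instigator as owner, then calls ClientLoadPopup, which activates the Signpost_LongText GUI module and passes the sign to its W_Sign_TextInput_Longly widget as content.
; SignText and LastEditor appear only in unexecuted nodes, and construction just calls the parent.
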(event `ClientLoadPopup`
  (bind _returnvalue (`GUIModuleController.ActivateModule` (`GUIModuleController.GetGUIModuleController`) "Signpost_LongText" true false))
  (bind _asw_sign_text_input_longly (cast `/Game/Mods/TDIRPAssets/Widgets/W_Sign_TextInput_Longly` _returnvalue)
    (:`then`
      (`/Game/Mods/TDIRPAssets/Widgets/W_Sign_TextInput_Longly.SetContent` _asw_sign_text_input_longly self))
    (:`CastFailed`
      (`KismetSystemLibrary.PrintString` "CastFailed"))))

(event `/Game/Systems/Building/Placeables/BP_Master_Placeables.Custom Interaction`
  (params (Instigator :type "PlayerController Object Reference") (HitIndex :type Integer) (IsOwner :type Boolean))
  (`self.SetOwner` Instigator)
  (`self.ClientLoadPopup`))

(fn `UserConstructionScript`
  (`parent.UserConstructionScript`))
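; BP_PL_SpinnyWheel is a placeable spinning wheel that shows a random number from 1 to 18 when activated.
; InteractableActivate calls PlaySpin, which plays a one-shot skeletal animation and picks the number independently of it.
; UpdatePlainTextFunction writes the number to the NumberDisplay widget through I_PlainText, ignoring its Widget input.
; Timed delays reveal the display after the spin, then hide it; Rotate is an empty stub.
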(event `self.ReceiveTick`
  (params (DeltaSeconds :type "Float (single-precision)")))

(event `InteractableInterface.InteractableActivate`
  (params (Component :type "PrimitiveComponent Object Reference") (Instigator :type "PlayerController Object Reference") (HitIndex :type Integer) (TriggeredFromRadialWheel :type Boolean))
  (`KismetSystemLibrary.PrintString` "Clicked")
  (`self.PlaySpin`))

(event `PlaySpin`
  (`SkeletalMeshComponent.PlayAnimation` (`self.SkeletalMesh`) "/Game/Mods/TDIRPAssets/3D/Placeables/Wheel/NewSM/SpinningWheel-42-v1_Anim.SpinningWheel-42-v1_Anim" false)
  (`self.UpdatePlainTextFunction` (`self.NumberDisplay`) (`KismetTextLibrary.Conv_StringToText` (`KismetStringLibrary.BuildString_Int` "" "" (`KismetMathLibrary.RandomIntegerInRange` 1 18) "!")))
  (`KismetSystemLibrary.Delay` 5.2)
  (`SceneComponent.SetHiddenInGame` (`self.NumberDisplay`) false false)
  (`KismetSystemLibrary.Delay` 10.0)
  (`SceneComponent.SetHiddenInGame` (`self.NumberDisplay`) true false))

(fn `Rotate`
  (params (Secs :type "Float (double-precision)" :default 0.0)))

(fn `UpdatePlainTextFunction`
  (params (Widget :type "WidgetComponent Object Reference") (NewText :type Text))
  (`KismetSystemLibrary.PrintString` "Begin Update Text" true false (struct :`G` 0.66 :`B` 1.0 :`A` 1.0) 14.0)
  (`KismetSystemLibrary.PrintString` "Updating the other widget" true false (struct :`R` 0.772115 :`B` 1.0 :`A` 1.0) 20.0)
  (bind _asi_plain_text (cast `/Game/Mods/TDIRPAssets/Widgets/I_PlainText` (`WidgetComponent.GetUserWidgetObject` (`self.NumberDisplay`))))
  (message `/Game/Mods/TDIRPAssets/Widgets/I_PlainText.UpdatePlainText` (`KismetSystemLibrary.Conv_InterfaceToObject` _asi_plain_text) NewText)
  (`KismetSystemLibrary.PrintString` "Didn't crash" true false)
  (`WidgetComponent.RequestRedraw` (`self.NumberDisplay`)))

(fn `UserConstructionScript`
  (`parent.UserConstructionScript`))
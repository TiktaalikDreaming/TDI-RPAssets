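; Siege engine projectile that launches along a firing rotation, with spin and in-air audio scaled to its initial speed.
; On first bounce the server damages avatars directly, or deals split health, armor-ignoring and explosive siege damage to other targets.
; Movement components are then removed, and a dedicated server spawns a lootable dummy projectile and disintegrates this one.
; Otherwise the mesh simulates physics until a looping velocity check finds it settled and destroys it.
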(event `InitProjectile`
  (bind _rotationrate (`self.RotationRate`))
  (bind _initialspeed (`self.InitialSpeed`))
  ;[1 0.6413 0.1882] Begin play
  (`KismetSystemLibrary.PrintString` (`KismetStringLibrary.Concat_StrStr` (`KismetTextLibrary.Conv_TextToString` (`KismetTextLibrary.AsDateTime_DateTime` (`KismetMathLibrary.UtcNow`))) "   Init Projectile") true false (struct :`G` 0.66 :`B` 1.0 :`A` 1.0) 10.0)
  (`self.SetLifeSpan` 120.0)
  (if (!= _initialspeed 0.0)
    (set `MovementComponent.Velocity` (`KismetMathLibrary.GreaterGreater_VectorRotator` (`KismetMathLibrary.MakeVector` _initialspeed) (`self.FiringRotation`)) (`self.ProjectileMovement`))
    (set `RotatingMovementComponent.RotationRate` (`KismetMathLibrary.MakeRotator` (* (`KismetMathLibrary.MapRangeClamped` (`self.InitialSpeed`) (`self.MinSpeed`) (`self.MaxSpeed`) 90.0 360.0) _rotationrate) (* _rotationrate (`KismetMathLibrary.RandomFloatInRange` -15.0 -15.0)) (* _rotationrate (`KismetMathLibrary.RandomFloatInRange` -15.0 15.0))) (`self.RotatingMovement`))
    (`ConanAudioComponent.SetVolumeMultiplier` (`self.InAir_Audio`) (`KismetMathLibrary.MapRangeClamped` (`self.InitialSpeed`) (`self.MinSpeed`) (`self.MaxSpeed`) 0.1 0.3))))

(event `CheckVelocity`
  (bind _staticmesh (`self.StaticMesh`))
  ;[1 0.6413 0.1882] Projectile impact handling
  ;;[0.02499 0.09524 0.16] Speed Checker
  (if (<= (`KismetMathLibrary.VSize` (`SceneComponent.GetComponentVelocity` (`self.StaticMesh`))) 60.0)
    (`|ExecutionSequence`
      (:`then_0`
        (`self.HasSettled`)
        (`/Engine/EditorBlueprintResources/StandardMacros.IsValid` _staticmesh
          (:`Is Valid`
            (`PrimitiveComponent.SetSimulatePhysics` _staticmesh false))))
      (:`then_1`
        (`KismetSystemLibrary.K2_ClearAndInvalidateTimerHandle` (`self.CheckVelocityTimer`))))))

(event `HasSettled`
  ;[1 0.6413 0.1882] Has Settled
  (if (not (`KismetSystemLibrary.IsDedicatedServer`))
    (`GameplayStatics.SpawnEmitterAtLocation` (`self.ImpactParticle`) (`SceneComponent.K2_GetComponentLocation` (`self.StaticMesh`))))
  (`self.K2_DestroyActor`))

(event `self.ProjectileMovement.OnProjectileBounce`
  (params (ImpactResult :type "HitResult Structure (by ref)") (ImpactVelocity :type "Vector Structure (by ref)"))
  (bind _rotatingmovement (`self.RotatingMovement`))
  ;[1 0.6413 0.1882] Projectile impact handling
  (bind _landedinwater (`self.CheckIfLandedInWater`))
  (if _landedinwater
    (`PrimitiveComponent.SetLinearDamping` (`self.StaticMesh`) 3.0)
    (else
      (`KismetSystemLibrary.PrintString` "Not in water" true false (struct :`G` 0.66 :`B` 1.0 :`A` 1.0) 10.0)))
  (`ConanAudioComponent.FadeOut` (`self.InAir_Audio`) 0.5 0.0)
  (`DreamworldBlueprints.PlaySoundAtLocation` (`self.Audio_Impact`) (`SceneComponent.K2_GetComponentLocation` (`self.StaticMesh`)))
  (`KismetSystemLibrary.PrintString` "Hit Something" true false (struct :`G` 0.66 :`B` 1.0 :`A` 1.0) 10.0)
  (`self.DoDamage` ImpactResult ImpactVelocity)
  (`MovementComponent.StopMovementImmediately` _rotatingmovement)
  (`MovementComponent.StopMovementImmediately` (`self.ProjectileMovement`))
  (`ActorComponent.K2_DestroyComponent` _rotatingmovement)
  (`ActorComponent.K2_DestroyComponent` (`self.ProjectileMovement`))
  (if (`KismetSystemLibrary.IsDedicatedServer`)
    (`self.TryToSpawnDummyProjectile` ImpactResult)
    (else
      (`ActorComponent.Deactivate` (`self.ParticleSystem`))
      (`self.SpawnEmitter` ImpactResult)))
  (if false
    (`self.Disintegrate` ImpactResult)
    (else
      (`PrimitiveComponent.SetSimulatePhysics` (`self.StaticMesh`) true)
      ;;[0.02499 0.09524 0.16] Speed Checker
      (bind _returnvalue (`KismetSystemLibrary.K2_SetTimerDelegate` (delegate `CheckVelocity`) 1.0 true))
      (set `self.CheckVelocityTimer` _returnvalue))))

(event `SpawnEmitter`
  (params (Hit :type "HitResult Structure"))
  ;[1 0.6413 0.1882] Spawn Emitter
  (if (`self.CanSpawnBounceParticle`)
    (set `self.CanSpawnBounceParticle` false)
    (`KismetSystemLibrary.K2_SetTimerDelegate` (delegate `ParticleCooldown`) 0.25)
    (`GameplayStatics.SpawnEmitterAtLocation` (`self.ImpactParticle`) (`.ImpactPoint` (`GameplayStatics.BreakHitResult` Hit)))))

(event `ParticleCooldown`
  ;[1 0.6413 0.1882] Spawn Emitter
  (set `self.CanSpawnBounceParticle` true))

(event `DoDamage`
  (params (Hit :type "HitResult Structure") (`Impact Velocity` :type "Vector Structure") (`PhysicsDamage?` :type Boolean))
  ;[1 0.6413 0.1882] Damage
  (if (`KismetSystemLibrary.IsServer`)
    (if (`self.CanDoDamage`)
      (bind _success (`self.TryToDamageAvatar` Hit))
      (if _success
        (`self.K2_DestroyActor`)
        (else
          (`self.ApplyDamage` Hit `PhysicsDamage?`))))))

(event `Disintegrate`
  (params (Hit :type "HitResult Structure"))
  ;[1 0.6413 0.1882] Disintegrate
  (`PrimitiveComponent.SetSimulatePhysics` (`self.StaticMesh`) false)
  (`SceneComponent.SetVisibility` (`self.StaticMesh`) false false)
  (if (not (`KismetSystemLibrary.IsDedicatedServer`))
    (`ActorComponent.Deactivate` (`self.ParticleSystem`)))
  (`KismetSystemLibrary.Delay` (`self.DisintegrateDestroyDelay`))
  (`self.K2_DestroyActor`))

(fn `ApplyDamage`
  (params (Hit :type "HitResult Structure") (PhysicsDamage :type Boolean))
  (locals (ModifiedBaseDamage :type "Float (double-precision)") (MinimumBaseDamage :type "Float (double-precision)") (SphereRadius :type "Float (double-precision)" :default 25.0) (OuterSphereRadius :type "Float (double-precision)" :default 100.0) (SphereRadius_Explosive :type "Float (double-precision)" :default 200.0) (OuterSphereRadius_Explosive :type "Float (double-precision)" :default 300.0) (`local Hit` :type "HitResult Structure") (`local PhysicsDamage` :type Boolean))
  (bind _returnvalue (`self.GetInstigatorController`))
  (bind (_local_hit_bblockinghit _local_hit_binitialoverlap _local_hit_time _local_hit_location _local_hit_impactpoint _local_hit_normal _local_hit_impactnormal _local_hit_physmat _local_hit_hitactor _local_hit_hitcomponent _local_hit_hitbonename _local_hit_hititem _local_hit_faceindex _local_hit_tracestart) (`GameplayStatics.BreakHitResult` (`local.local Hit`)))
  (bind _local_hit (`local.local Hit`))
  (bind (_local_hit_bblockinghit_2 _local_hit_binitialoverlap_2 _local_hit_time_2 _local_hit_location_2 _local_hit_impactpoint_2 _local_hit_normal_2 _local_hit_impactnormal_2 _local_hit_physmat_2 _local_hit_hitactor_2 _local_hit_hitcomponent_2 _local_hit_hitbonename_2 _local_hit_hititem_2 _local_hit_faceindex_2 _local_hit_tracestart_2) (`GameplayStatics.BreakHitResult` (`local.local Hit`)))
  (bind _returnvalue_2 (`KismetMathLibrary.FMax` (`local.MinimumBaseDamage`) (`local.ModifiedBaseDamage`)))
  (bind _returnvalue_3 (* _returnvalue_2 0.25))
  (bind _returnvalue_4 (`KismetMathLibrary.FMax` (* (`local.MinimumBaseDamage`) (`self.Siege Damage Multiplier`)) (* (`local.ModifiedBaseDamage`) (`self.Siege Damage Multiplier`))))
  (set `local.local Hit` Hit)
  (set `local.local PhysicsDamage` PhysicsDamage)
  (`|ExecutionSequence`
    (:`then_0`
      ;[1 0.6413 0.1882] Initialize Local Variables
      ;;[0.02499 0.09524 0.16] Set Damage
      (bind _output_get (set `local.ModifiedBaseDamage` (`self.GetModifiedImpactDamage` (`local.local PhysicsDamage`))))
      (bind _output_get_2 (set `local.MinimumBaseDamage` (* _output_get 0.25)))
      (`KismetSystemLibrary.PrintString` (`KismetStringLibrary.Concat_StrStr` "Min Base Damage determined to be" (`KismetStringLibrary.Conv_DoubleToString` _output_get_2)) true false (struct :`G` 0.66 :`B` 1.0 :`A` 1.0) 10.0))
    (:`then_1`
      ;[1 0.6413 0.1882] Do Health Damage
      (`GameplayStatics.ApplyPointDamage` _local_hit_hitactor (- _returnvalue_2 _returnvalue_3) _local_hit_tracestart _local_hit _returnvalue self "/Game/Systems/Progression/DmgTypeHealth_BP.DmgTypeHealth_BP_C")
      (`GameplayStatics.ApplyPointDamage` _local_hit_hitactor _returnvalue_3 _local_hit_tracestart _local_hit _returnvalue self "/Game/Systems/Progression/DmgTypeHealth_IgnoreArmor_BP.DmgTypeHealth_IgnoreArmor_BP_C")
      (`KismetSystemLibrary.PrintString` (`KismetStringLibrary.Concat_StrStr` "Base Health Damage " (`KismetStringLibrary.Conv_DoubleToString` _returnvalue_2)) true false (struct :`G` 0.66 :`B` 1.0 :`A` 1.0) 10.0))
    (:`then_2`
      ;[1 0.6413 0.1882] Do Explosive Damage
      (`GameplayStatics.ApplyPointDamage` _local_hit_hitactor_2 _returnvalue_4 _local_hit_tracestart_2 (`local.local Hit`) (`self.GetInstigatorController`) self "/Game/Systems/Combat/Dmg_Explosive.Dmg_Explosive_C")
      (`KismetSystemLibrary.PrintString` (`KismetStringLibrary.Concat_StrStr` "Siege Damage " (`KismetStringLibrary.Conv_DoubleToString` _returnvalue_4)) true false (struct :`G` 0.66 :`B` 1.0 :`A` 1.0) 10.0))))

(fn `CheckIfLandedInWater`
  (returns (LandedInWater :type Boolean))
  (bind _returnvalue (`SceneComponent.GetPhysicsVolume` (`self.StaticMesh`)))
  (bind _out_is_water (`/Game/Systems/MiscFunctions.IsWaterVolume` _returnvalue))
  (bind _out_is_water_2 (`/Game/Systems/MiscFunctions.IsWater` _returnvalue))
  (bind _output_get (set `self.LandedInWater` (or _out_is_water_2 _out_is_water)))
  (return _output_get))

(fn `GetAdjustedImpactPosition`
  (params (Hit :type "HitResult Structure"))
  (returns (ReturnValue :type "Vector Structure") (Success :type Boolean))
  (locals (LocalAdjustedPosition :type "Vector Structure") (LocalSuccess :type Boolean))
  (bind (_localhitresult_bblockinghit _localhitresult_binitialoverlap _localhitresult_time _localhitresult_location _localhitresult_impactpoint _localhitresult_normal _localhitresult_impactnormal _localhitresult_physmat _localhitresult_hitactor _localhitresult_hitcomponent) (`GameplayStatics.BreakHitResult` (`self.LocalHitResult`)))
  (`|ExecutionSequence`
    (:`then_0`
      ;[1 0.6413 0.1882] Initialize Local Variables
      (bind _output_get (set `self.LocalHitResult` Hit))
      (set `local.LocalAdjustedPosition` (`.ImpactPoint` (`GameplayStatics.BreakHitResult` _output_get))))
    (:`then_1`
      (`|ExecutionSequence`
        (:`then_0`
          ;[1 0.6413 0.1882] Try to find the staticmesh behind the Collision Box, in order to prevent floating arrows.
          (`/Engine/EditorBlueprintResources/StandardMacros.IsValid` _localhitresult_hitcomponent
            (:`Is Valid`
              (if (`|EnumEquality` (`PrimitiveComponent.GetCollisionObjectType` _localhitresult_hitcomponent) "ECC_GameTraceChannel2")
                (bind _outhit (`KismetSystemLibrary.LineTraceSingleForObjects` :`Start` (`local.LocalAdjustedPosition`) :`End` (- (`local.LocalAdjustedPosition`) (* (`KismetMathLibrary.Normal` (`self.GetVelocity`)) -100.0)) :`ObjectTypes` (`|MakeArray` "ObjectTypeQuery1" :!type "EObjectTypeQuery Enum") :`DrawTime` 1.0))
                (bind (_bblockinghit _binitialoverlap _time _location _impactpoint _normal _impactnormal _physmat _hitactor _hitcomponent) (`GameplayStatics.BreakHitResult` _outhit))
                (cast `MeshComponent` _hitcomponent
                  (:`then`
                    (set `local.LocalAdjustedPosition` _impactpoint))
                  (:`CastFailed`
                    (set `local.LocalSuccess` false)))))
            (:`Is Not Valid`
              (set `local.LocalSuccess` false))))
        (:`then_1`
          ;[1 0.6413 0.1882] Correct the positioning of the attached projectile.
          (set `local.LocalAdjustedPosition` (- (`local.LocalAdjustedPosition`) (* (`KismetMathLibrary.Normal` (`self.GetVelocity`)) (* (`.SphereRadius` (`KismetSystemLibrary.GetComponentBounds` (`self.StaticMesh`))) (- 2.0 0.3))))))))
    (:`then_2`
      (return (`local.LocalAdjustedPosition`) (`local.LocalSuccess`)))))

(fn `GetAttackerUniqueID`
  (returns (ReturnValue :type "UniqueID Object Reference"))
  (return (`self.AttackerUID`)))

(fn `GetModifiedImpactDamage`
  (params (Index :type Boolean))
  (returns (ReturnValue :type "Float (double-precision)"))
  (bind _basedamage (`self.BaseDamage`))
  (return (select `bool` Index :`false` _basedamage :`true` (* _basedamage (`KismetMathLibrary.MapRangeClamped` (`KismetMathLibrary.VSize` (`SceneComponent.GetComponentVelocity` (`self.StaticMesh`))) (`self.PhysicsMinimumVelocityToDoDamage`) (`self.PhysicsMaxVelocityToDoFullDamage`) 0.1 (`self.PhysicsDamageMod`))))))

(fn `IsPlayerDamage`
  (returns (ReturnValue :type Boolean))
  (return true))

(fn `IsThrallDamage`
  (returns (ReturnValue :type Boolean))
  (return false))

(fn `SpawnDummyProjectile`
  (params (HitResultFromProjectile :type "HitResult Structure") (ProjectileDummyLifetime :type "Float (double-precision)" :default 30.0) (IsLootable :type Boolean :default false) (ShouldBreakOnImpact :type Boolean :default false))
  (locals (LocalHitResultFromProjectile :type "HitResult Structure") (LocalProjectileDummyLifetime :type "Float (double-precision)") (LocalAdjustedPosition :type "Vector Structure") (localSpawnRotation :type "Rotator Structure") (LocalBreakOnImpact :type Boolean))
  (bind (_bblockinghit _binitialoverlap _time _location _impactpoint _normal _impactnormal) (`GameplayStatics.BreakHitResult` HitResultFromProjectile))
  (bind _velocity (`MovementComponent.Velocity` (`self.ProjectileMovement`)))
  (bind _returnvalue (`KismetMathLibrary.Normal` _velocity))
  (`|ExecutionSequence`
    (:`then_0`
      ;[1 0.6413 0.1882] Initialize Local Variables
      (set `local.LocalHitResultFromProjectile` HitResultFromProjectile)
      (set `local.LocalProjectileDummyLifetime` ProjectileDummyLifetime)
      (set `self.LocalIsLootable` IsLootable)
      (bind (_returnvalue_2 _success) (`self.GetAdjustedImpactPosition` (`local.LocalHitResultFromProjectile`)))
      (set `local.LocalAdjustedPosition` _returnvalue_2)
      (set `local.LocalBreakOnImpact` (or (not _success) ShouldBreakOnImpact)))
    (:`then_1`
      (`/Engine/EditorBlueprintResources/StandardMacros.IsValid` (`StaticMeshComponent.StaticMesh` (`self.StaticMesh`))
        (:`Is Valid`
          ;[0.02499 0.09524 0.16] Spawn the projectile only on the server, IF the projectile is going to be lootable.
          (if (and (`self.LocalIsLootable`) (not false))
            (if (`KismetSystemLibrary.IsServer`)
              ;[1 0.6413 0.1882] Spawn Projectile Dummy if there is a valid static mesh.
              (if (`ProjectileMovementComponent.bRotationFollowsVelocity` (`self.ProjectileMovement`)) :!label _label
                (set `local.localSpawnRotation` (`KismetMathLibrary.ComposeRotators` (`self.ProjectileOnGroundRotationOffset`) (`SceneComponent.K2_GetComponentRotation` (`self.StaticMesh`))))
                (else
                  (set `local.localSpawnRotation` (`KismetMathLibrary.ComposeRotators` (`self.ProjectileOnGroundRotationOffset`) (`KismetMathLibrary.MakeRotationFromAxes` _returnvalue (`KismetMathLibrary.Normal` (`KismetMathLibrary.Cross_VectorVector` _returnvalue _impactnormal)) _impactnormal)))))
              (`|SpawnActorFromClass` "/Game/Items/Weapons/BP_DummyProjectile.BP_DummyProjectile_C" (`KismetMathLibrary.MakeTransform` (`local.LocalAdjustedPosition`) (`local.localSpawnRotation`) (1.0 1.0 1.0)) "AlwaysSpawn" "OverrideRootScale" null HitResultFromProjectile (`StaticMeshComponent.StaticMesh` (`self.StaticMesh`)) 300.0 (`self.LocalIsLootable`) 22120272 false _velocity (`self.ItemDurability`)))
            (else
              (goto _label))))))))

(fn `TryToDamageAvatar`
  (params (HitInfo :type "HitResult Structure (by ref)"))
  (returns (Success :type Boolean))
  (locals (Local_HitInfo :type "HitResult Structure"))
  (bind (_local_hitinfo_bblockinghit _local_hitinfo_binitialoverlap _local_hitinfo_time _local_hitinfo_location _local_hitinfo_impactpoint _local_hitinfo_normal _local_hitinfo_impactnormal _local_hitinfo_physmat _local_hitinfo_hitactor) (`GameplayStatics.BreakHitResult` (`local.Local_HitInfo`)))
  (bind (_local_hitinfo_bblockinghit_2 _local_hitinfo_binitialoverlap_2 _local_hitinfo_time_2 _local_hitinfo_location_2 _local_hitinfo_impactpoint_2 _local_hitinfo_normal_2 _local_hitinfo_impactnormal_2 _local_hitinfo_physmat_2 _local_hitinfo_hitactor_2 _local_hitinfo_hitcomponent _local_hitinfo_hitbonename) (`GameplayStatics.BreakHitResult` (`local.Local_HitInfo`)))
  (`|ExecutionSequence`
    (:`then_0`
      ;[1 0.6413 0.1882] Initialize Local Variables
      (set `local.Local_HitInfo` HitInfo))
    (:`then_1`
      ;[0.62 0 0] Check: Did we hit an Avatar?
      (cast `AvatarCharacter` _local_hitinfo_hitactor_2
        (:`then`
          (`KismetSystemLibrary.PrintString` (`KismetStringLibrary.Concat_StrStr` "We hit " (`KismetSystemLibrary.GetDisplayName` _local_hitinfo_hitactor_2) " in the " (`KismetStringLibrary.Conv_NameToString` _local_hitinfo_hitbonename)))
          ;[1 0.6413 0.1882] Do damage
          (`GameplayStatics.ApplyPointDamage` _local_hitinfo_hitactor (`self.BaseDamage`) _local_hitinfo_impactpoint (`local.Local_HitInfo`) (`self.GetInstigatorController`) (`self.GetOwner`) "/Game/Systems/Progression/DmgTypeHealth_BP.DmgTypeHealth_BP_C")
          ;[0.62 0.1759 0.4784] Return: Success
          (return true))
        (:`CastFailed`
          ;[0.62 0.1759 0.4784] Return: Failure
          (return false))))))

(fn `TryToSpawnDummyProjectile`
  (params (HitResultFromProjectile :type "HitResult Structure"))
  (bind (_bblockinghit _binitialoverlap _time _location _impactpoint _normal _impactnormal _physmat _hitactor) (`GameplayStatics.BreakHitResult` (`self.LocalHitResult`)))
  (bind _returnvalue (or (`KismetSystemLibrary.DoesImplementInterface` (`self.GetOwner` _hitactor) "/Game/Systems/Interfaces/IsBaseBPCombatInterface.IsBaseBPCombatInterface_C") (`KismetSystemLibrary.DoesImplementInterface` _hitactor "/Game/Systems/Interfaces/IsBaseBPCombatInterface.IsBaseBPCombatInterface_C")))
  ;[0.02499 0.09524 0.16] Initial Checks
  (set `self.LocalHitResult` HitResultFromProjectile)
  (`|ExecutionSequence`
    (:`then_0`
      ;[1 0.6413 0.1882] Initialize Local Variables
      (set `self.LocalIsLootable` (not _returnvalue))
      (set `self.LocalIsCharacter` _returnvalue))
    (:`then_1`
      ;[1 0.6413 0.1882] If there is a mesh to show, spawn a dummy projectile and attach it to the hit actor.
      (`self.SpawnDummyProjectile` (`self.LocalHitResult`) 30.0 true (or (not false) (and (not (`self.LocalIsCharacter`)) true)))
      (`self.Disintegrate` (struct)))))

(fn `UserConstructionScript`)
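; BP_CatapultaInputComponent is the input component for a catapult siege weapon, relaying player input to the weapon held in its Ballista reference.
; Escape, crouch, jump and dismount presses all trigger dismounting.
; Turn and look axes, with separate controller variants, pass straight through for aiming or camera control.
; Releasing primary action fires, while pressing and releasing special action starts and stops charging.
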(event `InputAction|Escape`
  (params (Key :type "Key Structure" :default "AnyKey"))
  ;[1 1 1] Dismounting
  (:`Pressed`
    (`/Game/Systems/Building/Placeables/Trebuchet/Ballista/BP_Ballista_Complete.Input_Dismount` (`self.Ballista`) :!label _label)))

(event `InputAction|CrouchMode`
  (params (Key :type "Key Structure" :default "AnyKey"))
  ;[1 1 1] Dismounting
  (:`Pressed`
    (goto _label)))

(event `InputAction|Dismount`
  (params (Key :type "Key Structure" :default "AnyKey"))
  ;[1 1 1] Dismounting
  (:`Pressed`
    (goto _label)))

(event `InputAction|Jump`
  (params (Key :type "Key Structure" :default "AnyKey"))
  ;[1 1 1] Dismounting
  (:`Pressed`
    (goto _label)))

(event `InputAxis|Turn`
  (params (AxisValue :type "Float (single-precision)"))
  ;[1 1 1] Camera
  (`/Game/Systems/Building/Placeables/Trebuchet/Ballista/BP_Ballista_Complete.Input_Turn` (`self.Ballista`) AxisValue))

(event `InputAxis|LookUp`
  (params (AxisValue :type "Float (single-precision)"))
  ;[1 1 1] Camera
  (`/Game/Systems/Building/Placeables/Trebuchet/Ballista/BP_Ballista_Complete.Input_LookUp` (`self.Ballista`) AxisValue))

(event `InputAxis|TurnController`
  (params (AxisValue :type "Float (single-precision)"))
  ;[1 1 1] Camera
  (`/Game/Systems/Building/Placeables/Trebuchet/Ballista/BP_Ballista_Complete.Input_TurnController` (`self.Ballista`) AxisValue))

(event `InputAxis|LookUpController`
  (params (AxisValue :type "Float (single-precision)"))
  ;[1 1 1] Camera
  (`/Game/Systems/Building/Placeables/Trebuchet/Ballista/BP_Ballista_Complete.Input_LookUpController` (`self.Ballista`) AxisValue))

(event `InputAction|PrimaryActionV2`
  (params (Key :type "Key Structure" :default "AnyKey"))
  ;[1 1 1] Interaction
  (:`Released`
    (`/Game/Systems/Building/Placeables/Trebuchet/Ballista/BP_Ballista_Complete.Input_Fire` (`self.Ballista`))))

(event `InputAction|SpecialActionV2`
  (params (Key :type "Key Structure" :default "AnyKey"))
  (bind _ballista (`self.Ballista`))
  ;[1 1 1] Interaction
  (:`Pressed`
    (`/Game/Systems/Building/Placeables/Trebuchet/Ballista/BP_Ballista_Complete.Input_Start_Charge` _ballista))
  (:`Released`
    (`/Game/Systems/Building/Placeables/Trebuchet/Ballista/BP_Ballista_Complete.Input_Stop_Charge` _ballista)))
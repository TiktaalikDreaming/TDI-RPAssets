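; Catapult siege projectile that flies via projectile movement, with speed-scaled spin and in-air audio volume.
; On first bounce it plays impact effects, stops movement and applies server-side damage: avatar hits destroy it, others take health plus multiplied explosive damage.
; It then either disintegrates or switches to physics, damped in water, with a looping timer destroying it once it settles.
; Velocity-scaled physics damage exists, but the bounce path always uses base damage.
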(event `InitProjectile`
  (params (Start :type "Rotator Structure (by ref)"))
  (bind _rotationrate (`self.RotationRate`))
  (bind _initialspeed (`self.InitialSpeed`))
  ;[1 0.6413 0.1882] Begin play
  (`self.SetLifeSpan` 20.0)
  (if (!= _initialspeed 0.0)
    (set `MovementComponent.Velocity` (`KismetMathLibrary.GreaterGreater_VectorRotator` (`KismetMathLibrary.MakeVector` _initialspeed) Start) (`self.ProjectileMovement_0`))
    (set `RotatingMovementComponent.RotationRate` (`KismetMathLibrary.MakeRotator` (* (`KismetMathLibrary.MapRangeClamped` (`self.InitialSpeed`) (`self.MinSpeed`) (`self.MaxSpeed`) 90.0 360.0) _rotationrate) (* _rotationrate (`KismetMathLibrary.RandomFloatInRange` -1.0 1.0)) (* _rotationrate (`KismetMathLibrary.RandomFloatInRange` -1.0 1.0))) (`self.RotatingMovement`))
    (`ConanAudioComponent.SetVolumeMultiplier` (`self.InAir_Audio`) (`KismetMathLibrary.MapRangeClamped` (`self.InitialSpeed`) (`self.MinSpeed`) (`self.MaxSpeed`) 0.1 0.3))))

(event `CheckVelocity`
  (bind _staticmesh (`self.StaticMesh`))
  ;[1 0.6413 0.1882] Projectile impact handling
  ;;[0.02499 0.09524 0.16] Speed Checker
  (if (<= (`KismetMathLibrary.VSize` (`SceneComponent.GetComponentVelocity` (`self.StaticMesh`))) 60.0)
    (`|ExecutionSequence`
      (:`then_0`
        (`self.HasSettled`)
        (`/Engine/EditorBlueprintResources/StandardMacros.IsValid` _staticmesh
          (:`Is Valid`
            (`PrimitiveComponent.SetSimulatePhysics` _staticmesh false))))
      (:`then_1`
        (`KismetSystemLibrary.K2_ClearAndInvalidateTimerHandle` (`self.CheckVelocityTimer`))))))

(event `HasSettled`
  ;[1 0.6413 0.1882] Has Settled
  (if (not (`KismetSystemLibrary.IsDedicatedServer`))
    (`GameplayStatics.SpawnEmitterAtLocation` "/Game/Systems/Building/Placeables/Trebuchet/Trebuchet_V2/Particles/P_SiegeProjectile_Impact.P_SiegeProjectile_Impact" (`SceneComponent.K2_GetComponentLocation` (`self.StaticMesh`))))
  (`self.K2_DestroyActor`))

(event `self.ProjectileMovement_0.OnProjectileBounce`
  (params (ImpactResult :type "HitResult Structure (by ref)") (ImpactVelocity :type "Vector Structure (by ref)"))
  (bind _rotatingmovement (`self.RotatingMovement`))
  ;[1 0.6413 0.1882] Projectile impact handling
  (bind _landedinwater (`self.CheckIfLandedInWater`))
  (if _landedinwater
    (`PrimitiveComponent.SetLinearDamping` (`self.StaticMesh`) 3.0))
  (`ConanAudioComponent.FadeOut` (`self.InAir_Audio`) 0.5 0.0)
  (`DreamworldBlueprints.PlaySoundAtLocation` (`self.Audio_Impact`) (`SceneComponent.K2_GetComponentLocation` (`self.StaticMesh`)))
  (`self.DoDamage` ImpactResult ImpactVelocity)
  (`MovementComponent.StopMovementImmediately` _rotatingmovement)
  (`MovementComponent.StopMovementImmediately` (`self.ProjectileMovement_0`))
  (`ActorComponent.K2_DestroyComponent` _rotatingmovement)
  (`ActorComponent.K2_DestroyComponent` (`self.ProjectileMovement_0`))
  (if (not (`KismetSystemLibrary.IsDedicatedServer`))
    (`ActorComponent.Deactivate` (`self.ParticleSystem`))
    (`self.SpawnEmitter` ImpactResult))
  (if (`self.DisintegrateOnImpact`)
    (`self.Disintegrate` ImpactResult)
    (else
      (`PrimitiveComponent.SetSimulatePhysics` (`self.StaticMesh`) true)
      ;;[0.02499 0.09524 0.16] Speed Checker
      (bind _returnvalue (`KismetSystemLibrary.K2_SetTimerDelegate` (delegate `CheckVelocity`) 1.0 true))
      (set `self.CheckVelocityTimer` _returnvalue))))

(event `SpawnEmitter`
  (params (Hit :type "HitResult Structure"))
  ;[1 0.6413 0.1882] Spawn Emitter
  (if (`self.CanSpawnBounceParticle`)
    (set `self.CanSpawnBounceParticle` false)
    (`KismetSystemLibrary.K2_SetTimerDelegate` (delegate `ParticleCooldown`) 0.25)
    (`GameplayStatics.SpawnEmitterAtLocation` (`self.ImpactParticle`) (`.ImpactPoint` (`GameplayStatics.BreakHitResult` Hit)))))

(event `ParticleCooldown`
  ;[1 0.6413 0.1882] Spawn Emitter
  (set `self.CanSpawnBounceParticle` true))

(event `DoDamage`
  (params (Hit :type "HitResult Structure") (`Impact Velocity` :type "Vector Structure") (`PhysicsDamage?` :type Boolean))
  ;[1 0.6413 0.1882] Damage
  (`KismetSystemLibrary.PrintString` "DoDamange Start")
  (if (`KismetSystemLibrary.IsServer`)
    (if (`self.CanDoDamage`)
      (bind _success (`self.TryToDamageAvatar` Hit))
      (if _success
        (`self.K2_DestroyActor`)
        (else
          (`self.ApplyDamage` Hit `PhysicsDamage?`))))))

(event `Disintegrate`
  (params (Hit :type "HitResult Structure"))
  ;[1 0.6413 0.1882] Disintegrate
  (`PrimitiveComponent.SetSimulatePhysics` (`self.StaticMesh`) false)
  (`SceneComponent.SetVisibility` (`self.StaticMesh`) false false)
  (if (not (`KismetSystemLibrary.IsDedicatedServer`))
    (`ActorComponent.Deactivate` (`self.ParticleSystem`)))
  (`KismetSystemLibrary.Delay` (`self.DisintegrateDestroyDelay`))
  (`self.K2_DestroyActor`))

(fn `ApplyDamage`
  (params (Hit :type "HitResult Structure") (PhysicsDamage :type Boolean))
  (locals (ModifiedBaseDamage :type "Float (double-precision)") (MinimumBaseDamage :type "Float (double-precision)" :default 300.0) (SphereRadius :type "Float (double-precision)" :default 25.0) (OuterSphereRadius :type "Float (double-precision)" :default 100.0) (SphereRadius_Explosive :type "Float (double-precision)" :default 200.0) (OuterSphereRadius_Explosive :type "Float (double-precision)" :default 300.0) (`local Hit` :type "HitResult Structure") (`local PhysicsDamage` :type Boolean))
  (bind (_local_hit_bblockinghit _local_hit_binitialoverlap _local_hit_time _local_hit_location _local_hit_impactpoint _local_hit_normal _local_hit_impactnormal _local_hit_physmat _local_hit_hitactor _local_hit_hitcomponent _local_hit_hitbonename _local_hit_hititem _local_hit_faceindex _local_hit_tracestart) (`GameplayStatics.BreakHitResult` (`local.local Hit`)))
  (bind (_local_hit_bblockinghit_2 _local_hit_binitialoverlap_2 _local_hit_time_2 _local_hit_location_2 _local_hit_impactpoint_2 _local_hit_normal_2 _local_hit_impactnormal_2 _local_hit_physmat_2 _local_hit_hitactor_2 _local_hit_hitcomponent_2 _local_hit_hitbonename_2 _local_hit_hititem_2 _local_hit_faceindex_2 _local_hit_tracestart_2) (`GameplayStatics.BreakHitResult` (`local.local Hit`)))
  (set `local.local Hit` Hit)
  (set `local.local PhysicsDamage` PhysicsDamage)
  (`KismetSystemLibrary.PrintString` "Calculating Damage")
  (`|ExecutionSequence`
    (:`then_0`
      ;[1 0.6413 0.1882] Initialize Local Variables
      ;;[0.02499 0.09524 0.16] Set Damage
      (bind _output_get (set `local.ModifiedBaseDamage` (`self.GetModifiedImpactDamage` (`local.local PhysicsDamage`))))
      (set `local.MinimumBaseDamage` (* _output_get 0.25)))
    (:`then_1`
      ;[1 0.6413 0.1882] Do Health Damage
      (`GameplayStatics.ApplyPointDamage` _local_hit_hitactor (`KismetMathLibrary.FMax` (`local.MinimumBaseDamage`) (`local.ModifiedBaseDamage`)) _local_hit_tracestart (`local.local Hit`) (`self.GetInstigatorController`) self "/Game/Systems/Progression/DmgTypeHealth_BP.DmgTypeHealth_BP_C"))
    (:`then_2`
      ;[1 0.6413 0.1882] Do Explosive Damage
      (`GameplayStatics.ApplyPointDamage` _local_hit_hitactor_2 (`KismetMathLibrary.FMax` (* (`local.MinimumBaseDamage`) (`self.Siege Damage Multiplier`)) (* (`local.ModifiedBaseDamage`) (`self.Siege Damage Multiplier`))) _local_hit_tracestart_2 (`local.local Hit`) (`self.GetInstigatorController`) self "/Game/Systems/Combat/Dmg_Explosive.Dmg_Explosive_C"))))

(fn `CheckIfLandedInWater`
  (returns (LandedInWater :type Boolean))
  (bind _returnvalue (`SceneComponent.GetPhysicsVolume` (`self.StaticMesh`)))
  (bind _out_is_water (`/Game/Systems/MiscFunctions.IsWaterVolume` _returnvalue))
  (bind _out_is_water_2 (`/Game/Systems/MiscFunctions.IsWater` _returnvalue))
  (bind _output_get (set `self.LandedInWater` (or _out_is_water_2 _out_is_water)))
  (return _output_get))

(fn `GetAttackerUniqueID`
  (returns (ReturnValue :type "UniqueID Object Reference"))
  (return (`self.AttackerUID_0`)))

(fn `GetModifiedImpactDamage`
  (params (Index :type Boolean))
  (returns (ReturnValue :type "Float (double-precision)"))
  (bind _basedamage (`self.BaseDamage`))
  (return (select `bool` Index :`false` _basedamage :`true` (* _basedamage (`KismetMathLibrary.MapRangeClamped` (`KismetMathLibrary.VSize` (`SceneComponent.GetComponentVelocity` (`self.StaticMesh`))) (`self.PhysicsMinimumVelocityToDoDamage`) (`self.PhysicsMaxVelocityToDoFullDamage`) 0.1 (`self.PhysicsDamageMod`))))))

(fn `IsPlayerDamage`
  (returns (ReturnValue :type Boolean))
  (return true))

(fn `IsThrallDamage`
  (returns (ReturnValue :type Boolean))
  (return false))

(fn `TryToDamageAvatar`
  (params (HitInfo :type "HitResult Structure (by ref)"))
  (returns (Success :type Boolean))
  (locals (Local_HitInfo :type "HitResult Structure"))
  (bind (_local_hitinfo_bblockinghit _local_hitinfo_binitialoverlap _local_hitinfo_time _local_hitinfo_location _local_hitinfo_impactpoint _local_hitinfo_normal _local_hitinfo_impactnormal _local_hitinfo_physmat _local_hitinfo_hitactor) (`GameplayStatics.BreakHitResult` (`local.Local_HitInfo`)))
  (bind (_local_hitinfo_bblockinghit_2 _local_hitinfo_binitialoverlap_2 _local_hitinfo_time_2 _local_hitinfo_location_2 _local_hitinfo_impactpoint_2 _local_hitinfo_normal_2 _local_hitinfo_impactnormal_2 _local_hitinfo_physmat_2 _local_hitinfo_hitactor_2) (`GameplayStatics.BreakHitResult` (`local.Local_HitInfo`)))
  (`|ExecutionSequence`
    (:`then_0`
      ;[1 0.6413 0.1882] Initialize Local Variables
      (set `local.Local_HitInfo` HitInfo))
    (:`then_1`
      ;[0.62 0 0] Check: Did we hit an Avatar?
      (cast `AvatarCharacter` _local_hitinfo_hitactor_2
        (:`then`
          ;[1 0.6413 0.1882] Do damage
          (`GameplayStatics.ApplyPointDamage` _local_hitinfo_hitactor (`self.BaseDamage`) _local_hitinfo_impactpoint (`local.Local_HitInfo`) (`self.GetInstigatorController`) (`self.GetOwner`) "/Game/Systems/Progression/DmgTypeHealth_BP.DmgTypeHealth_BP_C")
          ;[0.62 0.1759 0.4784] Return: Success
          (return true))
        (:`CastFailed`
          ;[0.62 0.1759 0.4784] Return: Failure
          (return false))))))

(fn `UserConstructionScript`)
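; Siege ballista Blueprint that alternates between loading and firing when a player interacts with it.
; Interaction plays the load animation if already fired, becoming ready after a fixed delay, or fires if loaded, playing the fire animation and triggering a multicast sound component.
; IsFired and IsLoaded gate the cycle, ignoring interaction during reload; no projectile is spawned here.
; A point-damage gong-sphere hit check leads to no action, and debug prints remain.
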(event `self.ReceivePointDamage`
  (params (Damage :type "Float (single-precision)") (DamageType :type "DamageType Object Reference") (HitLocation :type "Vector Structure") (HitNormal :type "Vector Structure") (HitComponent :type "PrimitiveComponent Object Reference") (BoneName :type Name) (ShotFromDirection :type "Vector Structure") (InstigatedBy :type "Controller Object Reference") (DamageCauser :type "Actor Object Reference") (HitInfo :type "HitResult Structure (by ref)"))
  (bind _checkgongcontactsphere (`self.CheckGongContactSphere`))
  (`parent.ReceivePointDamage` Damage DamageType HitLocation HitNormal HitComponent BoneName ShotFromDirection InstigatedBy DamageCauser HitInfo)
  (cast `PlayerController` InstigatedBy)
  (if (< (`KismetMathLibrary.VSize` (- HitLocation (`SceneComponent.K2_GetComponentLocation` _checkgongcontactsphere))) (`SphereComponent.SphereRadius` _checkgongcontactsphere))
    _))

(event `InteractableInterface.InteractableActivate`
  (params (Component :type "PrimitiveComponent Object Reference") (Instigator :type "PlayerController Object Reference") (HitIndex :type Integer) (TriggeredFromRadialWheel :type Boolean))
  (`KismetSystemLibrary.PrintString` "Interactededed" true true (struct :`G` 0.66 :`B` 1.0 :`A` 1.0) 6.0)
  (if (`self.IsFired`)
    (`self.LoadCatapulta`)
    (elif (`self.IsLoaded`)
      (`self.FireCatapulta`))))

(event `LoadCatapulta`
  (bind _skeletalmesh (`self.SkeletalMesh`))
  (set `self.IsFired` false)
  (`SkeletalMeshComponent.SetAnimation` _skeletalmesh "/Game/Mods/TDIRPAssets/3D/Siege/ballista_Anim_load.ballista_Anim_load")
  (`SkeletalMeshComponent.PlayAnimation` _skeletalmesh "/Game/Mods/TDIRPAssets/3D/Siege/ballista_Anim_load.ballista_Anim_load" false)
  (`KismetSystemLibrary.Delay` 20.0)
  (set `self.IsLoaded` true)
  (set `self.IsFired` false))

(event `FireCatapulta`
  (bind _skeletalmesh (`self.SkeletalMesh`))
  (`SkeletalMeshComponent.SetAnimation` _skeletalmesh "/Game/Mods/TDIRPAssets/3D/Siege/ballista_Anim_fire.ballista_Anim_fire")
  (`SkeletalMeshComponent.PlayAnimation` _skeletalmesh "/Game/Mods/TDIRPAssets/3D/Siege/ballista_Anim_fire.ballista_Anim_fire" false)
  (set `self.IsLoaded` false)
  (set `self.IsFired` true)
  (`KismetSystemLibrary.PrintString` "PlayPew" true true (struct :`R` 1.0 :`G` 0.486127 :`A` 1.0) 6.0)
  (`self.PlayPew`))

(event `PlayPew`
  (`/Game/Systems/Building/BuildingActorComponents/00_BP_SC_Building_MasterSceneComponent.InteractableActivate` (`self.BP_BSC_MulticastSound`) null null 0 false))

(fn `UserConstructionScript`
  (`parent.UserConstructionScript`))
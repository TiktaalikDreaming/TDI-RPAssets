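; Base Blueprint for torsion siege projectiles, driving tracer trail visuals that scale with replicated power charge.
; Effect scaling feeds direction, position and camera location into dynamic trail materials, then fades opacity by timeline.
; Impact starts a second, client-side fade that multiplies into that opacity.
; A charge curve sets ring size, glow, material scale and distortion; near-full charge swaps the sound transmitter, and mounted use is disallowed.
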(event `self.StartEffectScaling`
  (bind _tracerparticlesystem (`self.TracerParticleSystem`))
  (for _index (range 5)
    (bind _returnvalue (`PrimitiveComponent.CreateDynamicMaterialInstance` _tracerparticlesystem _index (`PrimitiveComponent.GetMaterial` _tracerparticlesystem _index)))
    (`MaterialInstanceDynamic.SetVectorParameterValue` _returnvalue "td" (`KismetMathLibrary.Conv_VectorToLinearColor` (`self.GetActorForwardVector` self)))
    (`MaterialInstanceDynamic.SetVectorParameterValue` _returnvalue "tp" (`KismetMathLibrary.Conv_VectorToLinearColor` (`self.K2_GetActorLocation` self)))
    (`MaterialInstanceDynamic.SetVectorParameterValue` _returnvalue "cp" (`KismetMathLibrary.Conv_VectorToLinearColor` (`PlayerCameraManager.GetCameraLocation` (`GameplayStatics.GetPlayerCameraManager` 0)))))
  (bind (_direction _opacity) (`Timeline|FadeTrail` :!via `PlayFromStart`)
    (:`Update`
      (`ParticleSystemComponent.SetFloatParameter` (`self.TracerParticleSystem`) "opacity" (* _opacity (`self.ImpactFadeAmount`))))))

(event `self.StopProjectileInternal`
  (params (Hit :type "HitResult Structure"))
  (`parent.StopProjectileInternal` Hit)
  (if (not (`KismetSystemLibrary.IsDedicatedServer`))
    (`/Engine/EditorBlueprintResources/StandardMacros.DoOnce` false
      (:`Completed`
        (bind (_direction _opacity) (`Timeline|FadeTrailOnImpact` :!via `PlayFromStart`)
          (:`Update`
            (set `self.ImpactFadeAmount` _opacity)))))))

(event `self.OnRep_PowerChargeMod`
  (bind _tracerparticlesystem (`self.TracerParticleSystem`))
  (bind _tracerparticlesystem_2 (`self.TracerParticleSystem`))
  (bind _returnvalue (`CurveFloat.GetFloatValue` (`self.PowerChargeTrailSize`) (`self.PowerChargeMod`)))
  (bind _returnvalue_2 (* _returnvalue 0.003))
  (`/Engine/EditorBlueprintResources/StandardMacros.IsValid` _tracerparticlesystem_2
    (:`Is Valid`
      (`ParticleSystemComponent.SetFloatParameter` _tracerparticlesystem_2 "ringsize" _returnvalue)
      (for _index (range 4)
        (bind _returnvalue_3 (`PrimitiveComponent.CreateDynamicMaterialInstance` _tracerparticlesystem _index (`PrimitiveComponent.GetMaterial` _tracerparticlesystem _index)))
        (`MaterialInstanceDynamic.SetScalarParameterValue` _returnvalue_3 "endscale" (+ _returnvalue_2 0.015))
        (`MaterialInstanceDynamic.SetScalarParameterValue` _returnvalue_3 "scale" (+ _returnvalue_2 0.005))
        (`MaterialInstanceDynamic.SetScalarParameterValue` _returnvalue_3 "distort" (`KismetMathLibrary.Lerp` 0.6 0.1 _returnvalue)))
      (`ParticleSystemComponent.SetFloatParameter` _tracerparticlesystem "glow" (+ (* _returnvalue 3.0) 1.0)))))

(fn `CanUseWhenMounted`
  (params (Mount :type "ConanCharacter Object Reference"))
  (returns (ReturnValue :type Boolean))
  (return false))

(fn `GetSoundTransmitter`
  (returns (SoundTransmitter :type "/Game/Sound/Tables/SoundTransmitterType Enum"))
  (if (>= (`self.PowerChargeMod`) 0.9)
    (return "NewEnumerator47")
    (else
      (return (`parent.GetSoundTransmitter`)))))

(fn `UserConstructionScript`
  (bind _tracerparticlesystem (`self.TracerParticleSystem`))
  (`parent.UserConstructionScript`)
  (`/Engine/EditorBlueprintResources/StandardMacros.IsValid` _tracerparticlesystem
    (:`Is Valid`
      (`ParticleSystemComponent.SetFloatParameter` _tracerparticlesystem "ringsize" (`CurveFloat.GetFloatValue` (`self.PowerChargeTrailSize`) (`self.PowerChargeMod`))))))
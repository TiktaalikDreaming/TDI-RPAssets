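; A placeable Conan Exiles siege catapult that players aim, load and fire as a bolt thrower.
; Server-side interaction routes the beam to a timed reload or firing, pointers to yaw and clamped tilt, and base parts to storage.
; Firing consumes an inventory bolt and spawns a projectile; dry firing damages the catapult itself.
; Inventory changes toggle the visible bolt when loaded, while a proximity widget shows rotation and elevation to local players.
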(event `InteractableInterface.InteractableActivate`
  (params (Component :type "PrimitiveComponent Object Reference") (Instigator :type "PlayerController Object Reference") (HitIndex :type Integer) (TriggeredFromRadialWheel :type Boolean))
  (bind _returnvalue (`SceneComponent.K2_GetComponentToWorld` (`self.Arrow`)))
  ;[1 1 1] Interactions
  (if (`KismetSystemLibrary.IsServer`)
    (`KismetSystemLibrary.PrintString` (`KismetStringLibrary.Concat_StrStr` "Interactededed" (`KismetStringLibrary.Conv_ObjectToString` Component) "  at " (`KismetStringLibrary.TimeSecondsToString` (`.PartialSeconds` (`GameplayStatics.GetAccurateRealTime`)))) true false (struct :`G` 0.66 :`B` 1.0 :`A` 1.0) 6.0)
    (if (== Component (`self.BoxLongBeam`))
      (if (`self.IsFired`)
        (`self.LoadCatapulta`)
        (elif (`self.IsLoaded`)
          (`self.FireCatapulta` _returnvalue (.rotation _returnvalue))
          (`self.PlayPew`)))
      (elif (== Component (`self.PointerCW`))
        (`self.Turn CW`)
        (`self.UpdateText` (`self.NewWidget`) (`self.CurrrentSetting`) :!label _label)
        (elif (== Component (`self.PointerCCW`))
          (`self.Turn CCW`)
          (goto _label)
          (elif (== Component (`self.PointerDown`))
            (`self.Tilt Down`)
            (goto _label)
            (elif (== Component (`self.PointerUp`))
              (`self.Tilt Up`)
              (goto _label)
              (elif (== Component (`self.BaseCol`))
                (`InteractableInterface.InteractableActivate` (`self.BP_BAC_Storage`) null Instigator 0 false :!label _label_2)
                (elif (== Component (`self.CatapultaStand`))
                  (goto _label_2))))))))))

(event `LoadCatapulta`
  (bind _mainbody (`self.MainBody`))
  ;[1 1 1] Load Up
  (set `self.IsFired` false)
  (`|ExecutionSequence`
    (:`then_0`
      (`SkeletalMeshComponent.SetAnimation` _mainbody "/Game/Mods/TDIRPAssets/3D/Siege/SK_Catapulta6_Anim_2.SK_Catapulta6_Anim_2")
      (`SkeletalMeshComponent.PlayAnimation` _mainbody "/Game/Mods/TDIRPAssets/3D/Siege/SK_Catapulta6_Anim_2.SK_Catapulta6_Anim_2" false))
    (:`then_1`
      (`KismetSystemLibrary.PrintString` "Loading please wait" true false (struct :`R` 1.0 :`G` 0.203596 :`A` 1.0) 20.0)
      (`KismetSystemLibrary.Delay` 20.0)
      (set `self.IsLoaded` true)
      (set `self.IsFired` false)
      (bind _hasammo_ (`self.Check Ammo` false))
      (if _hasammo_
        (`SceneComponent.SetHiddenInGame` (`self.BoltPlacement`) false false)
        (set `self.HasBolt` true)))))

(event `FireCatapulta`
  (params (FireTransform :type "Transform Structure") (Direction :type "Rotator Structure"))
  (bind _mainbody (`self.MainBody`))
  (bind _instigator (`self.Instigator`))
  ;[1 1 1] Fireing things
  (`SkeletalMeshComponent.SetAnimation` _mainbody "/Game/Mods/TDIRPAssets/3D/Siege/SK_Catapulta6_Anim.SK_Catapulta6_Anim")
  (`SkeletalMeshComponent.PlayAnimation` _mainbody "/Game/Mods/TDIRPAssets/3D/Siege/SK_Catapulta6_Anim.SK_Catapulta6_Anim" false)
  (set `self.IsLoaded` false)
  (set `self.IsFired` true)
  (`KismetSystemLibrary.PrintString` "PlayPew" true false (struct :`R` 1.0 :`G` 0.486127 :`A` 1.0) 6.0)
  (`self.PlayPew`)
  (bind _hasammo_ (`self.Check Ammo` true))
  (if _hasammo_
    (`KismetSystemLibrary.PrintString` "Bolt goes pew" true false)
    (`SceneComponent.SetHiddenInGame` (`self.BoltPlacement`) true false)
    (set `self.HasBolt` false)
    ;[1 1 1] Generate Projectile
    (`KismetSystemLibrary.PrintString` (`KismetStringLibrary.Conv_TransformToString` FireTransform) true false (struct :`R` 1.0 :`G` 0.089986 :`B` 0.331828 :`A` 1.0) 12.0 :!label _label_3)
    (bind _returnvalue (`|SpawnActorFromClass` "/Game/Mods/TDIRPAssets/3D/Siege/BP_V2_Engine_Projectile_6.BP_V2_Engine_Projectile_6_C" FireTransform "Undefined" "OverrideRootScale" _instigator 12000.0 9000.0 13000.0 1.1 0.0 _instigator))
    (`KismetSystemLibrary.PrintString` (`KismetStringLibrary.Concat_StrStr` (`KismetTextLibrary.Conv_TextToString` (`KismetTextLibrary.AsDateTime_DateTime` (`KismetMathLibrary.UtcNow`))) " Dart Actor Spawned") true false (struct :`G` 0.66 :`B` 1.0 :`A` 1.0) 10.0)
    (bind _uniqueid (message `/Game/Systems/Interfaces/BasePlayerCharInterface.GetUniqueID` _instigator))
    (set `/Game/Mods/TDIRPAssets/3D/Siege/BP_V2_Engine_Projectile_6.InitialSpeed` 13000.0 _returnvalue)
    (set `/Game/Mods/TDIRPAssets/3D/Siege/BP_V2_Engine_Projectile_6.MinSpeed` 300.0 _returnvalue)
    (set `/Game/Mods/TDIRPAssets/3D/Siege/BP_V2_Engine_Projectile_6.MaxSpeed` 15000.0 _returnvalue)
    (set `/Game/Mods/TDIRPAssets/3D/Siege/BP_V2_Engine_Projectile_6.FiringRotation` Direction _returnvalue)
    (set `/Game/Mods/TDIRPAssets/3D/Siege/BP_V2_Engine_Projectile_6.AttackerUID` _uniqueid _returnvalue)
    (set `/Game/Mods/TDIRPAssets/3D/Siege/BP_V2_Engine_Projectile_6.StaticMesh` (`self.BoltPlacement`) _returnvalue)
    (`KismetSystemLibrary.PrintString` (`KismetStringLibrary.Concat_StrStr` (`KismetTextLibrary.Conv_TextToString` (`KismetTextLibrary.AsDateTime_DateTime` (`KismetMathLibrary.UtcNow`))) "All set, init-ing") true false (struct :`G` 0.66 :`B` 1.0 :`A` 1.0) 10.0)
    (`/Game/Mods/TDIRPAssets/3D/Siege/BP_V2_Engine_Projectile_6.InitProjectile` _returnvalue)
    (else
      (`KismetSystemLibrary.PrintString` "no bolt but pew-ish" true false)
      (`GameplayStatics.ApplyDamage` self 4700.0 null null "/Game/Systems/Combat/Dmg_Explosive.Dmg_Explosive_C"))))

(event `FireOutBolt`
  (params (FireTransfrom :type "Transform Structure"))
  ;[1 1 1] Generate Projectile
  (goto _label_3))

(event `PlayPew`
  ;[1 1 1] Sounds
  (`DreamworldBlueprints.SpawnSoundAttached` "/Game/Mods/TDIRPAssets/3D/Siege/sfx_fire_pew.sfx_fire_pew" (`self.Pew`)))

(event `Turn CW`
  (bind _returnvalue (`KismetStringLibrary.Concat_StrStr` "Rotation: " (`KismetStringLibrary.Conv_DoubleToString` (`self.Heading`)) "\n" "Elevation: " (`KismetStringLibrary.Conv_DoubleToString` (`self.Elevation`))))
  ;[1 1 1] Aiming
  (`SceneComponent.K2_AddLocalRotation` (`self.CatapultaPivot`) (struct :`Yaw` -1.5) false false)
  (set `self.Heading` (+ (`self.Heading`) -1.5))
  (`KismetSystemLibrary.PrintString` _returnvalue true false (struct :`R` 0.547264 :`G` 1.0 :`B` 0.826259 :`A` 1.0) 6.0 :!label _label_4)
  (bind _output_get (set `self.CurrrentSetting` (`KismetTextLibrary.Conv_StringToText` _returnvalue) :!label _label_5))
  (`self.UpdateText` (`self.NewWidget`) _output_get))

(event `Turn CCW`
  ;[1 1 1] Aiming
  (`SceneComponent.K2_AddLocalRotation` (`self.CatapultaPivot`) (struct :`Yaw` 1.5) false false)
  (set `self.Heading` (+ (`self.Heading`) 1.5))
  (goto _label_4))

(event `Tilt Up`
  (bind _elevation (`self.Elevation`))
  ;[1 1 1] Aiming
  (if (not (> _elevation 20.0))
    (`SceneComponent.K2_AddLocalRotation` (`self.MainBody`) (struct :`Pitch` 1.0) false false)
    (set `self.Elevation` (+ _elevation 1.0))
    (`KismetSystemLibrary.PrintString` (`KismetStringLibrary.Concat_StrStr` "Rotation: " (`KismetStringLibrary.Conv_DoubleToString` (`self.Heading`)) "\n" "Elevation: " (`KismetStringLibrary.Conv_DoubleToString` _elevation)) true false (struct :`R` 0.547264 :`G` 1.0 :`B` 0.826259 :`A` 1.0) 6.0 :!label _label_6)
    (goto _label_5)))

(event `Tilt Down`
  (bind _elevation (`self.Elevation`))
  ;[1 1 1] Aiming
  (if (> _elevation -20.0)
    (`SceneComponent.K2_AddLocalRotation` (`self.MainBody`) (struct :`Pitch` -1.0) false false)
    (set `self.Elevation` (+ _elevation -1.0))
    (goto _label_6)))

(event `self.ReceiveBeginPlay`
  (bind _placeableinventory (`self.PlaceableInventory`))
  ;[1 1 1] Construction
  (`parent.ReceiveBeginPlay`)
  (if (`KismetSystemLibrary.IsServer`)
    (add `ItemInventory.SignalItemAdded` _placeableinventory (delegate `ItemAdded`))
    (add `ItemInventory.SignalItemRemoved` _placeableinventory (delegate `ItemRemoved`))
    (add `ItemInventory.SignalItemFloatStatChanged` _placeableinventory (delegate `ItemChanged`))))

(event `ItemChanged`
  (params (item :type "GameItem Object Reference") (statID :type "EItemFloatStatID Enum") (statValue :type "Float (double-precision)") (deltaValue :type "Float (double-precision)"))
  ;[1 1 1] Construction
)

(event `ItemAdded`
  (params (index :type Integer) (item :type "GameItem Object Reference") (srcInventory :type "ItemInventory Object Reference") (srcIndex :type Integer))
  (bind _boltplacement (`self.BoltPlacement`))
  ;[1 1 1] Construction
  (`KismetSystemLibrary.PrintString` "ItemAdded" true false (struct :`G` 0.66 :`B` 1.0 :`A` 1.0) 10.0)
  (if (`self.IsLoaded`) :!label _label_7
    (bind _hasammo_ (`self.Check Ammo` false))
    (if _hasammo_
      (`SceneComponent.SetHiddenInGame` _boltplacement false false)
      (set `self.HasBolt` true)
      (else
        (`SceneComponent.SetHiddenInGame` _boltplacement true false)
        (set `self.HasBolt` false)))))

(event `ItemRemoved`
  (params (index :type Integer) (item :type "GameItem Object Reference") (dstInventory :type "ItemInventory Object Reference") (dstIndex :type Integer))
  ;[1 1 1] Construction
  (`KismetSystemLibrary.PrintString` "ItemRemoved" true false (struct :`G` 0.66 :`B` 1.0 :`A` 1.0) 10.0)
  (goto _label_7))

(event `self.HoverArea.OnComponentBeginOverlap`
  (params (OverlappedComponent :type "PrimitiveComponent Object Reference") (OtherActor :type "Actor Object Reference") (OtherComp :type "PrimitiveComponent Object Reference") (OtherBodyIndex :type Integer) (bFromSweep :type Boolean) (SweepResult :type "HitResult Structure (by ref)"))
  (bind _newwidget (`self.NewWidget`))
  (`KismetSystemLibrary.PrintString` "Overlap Base" true false (struct :`G` 0.66 :`B` 1.0 :`A` 1.0) 20.0)
  (`self.CheckLocal` OtherActor
    (:`Local`
      (`self.CheckPlayer` OtherActor
        (:`true`
          (`self.UpdateText` _newwidget (`self.CurrrentSetting`))
          (`WidgetComponent.RequestRedraw` _newwidget)
          (`SceneComponent.SetHiddenInGame` _newwidget false false))))))

(event `self.HoverArea.OnComponentEndOverlap`
  (params (OverlappedComponent :type "PrimitiveComponent Object Reference") (OtherActor :type "Actor Object Reference") (OtherComp :type "PrimitiveComponent Object Reference") (OtherBodyIndex :type Integer))
  (bind _newwidget (`self.NewWidget`))
  (`KismetSystemLibrary.PrintString` "Stop Overlap" true false (struct :`G` 0.66 :`B` 1.0 :`A` 1.0) 20.0)
  (`self.CheckLocal` OtherActor
    (:`Local`
      (`self.CheckPlayer` OtherActor
        (:`true`
          _)
        (:`false`
          _)))
    (:`NotLocal`
      _)
    (:`Faulty`
      _))
  (message `/Game/Mods/TDIRPAssets/Widgets/I_Siege_Aim.HideText` _newwidget)
  (`KismetSystemLibrary.Delay` 8.0)
  (`SceneComponent.SetHiddenInGame` _newwidget true false))

(fn `Check Ammo`
  (params (Consume :type Boolean))
  (returns (`HasAmmo?` :type Boolean))
  (locals (`Bolt ID` :type Integer :default 22120272))
  (bind _bolt_id (`local.Bolt ID`))
  (if (`ItemInventory.HasItemByTemplateID` (`self.PlaceableInventory`) _bolt_id 1)
    (if Consume
      (`ItemInventory.DeleteItemsByTemplate` (`self.PlaceableInventory`) _bolt_id "consumed" 1)
      (return true)
      (else
        (return true)))
    (else
      (return false))))

(fn `Fade Text`
  (params (Widget :type "WidgetComponent Object Reference"))
  (message `/Game/Mods/TDIRPAssets/Widgets/I_Siege_Aim.HideText` Widget))

(fn `UpdateText`
  (params (Widget :type "WidgetComponent Object Reference") (`Display Text` :type Text))
  (`KismetSystemLibrary.PrintString` "Begin Update Text" true false (struct :`G` 0.66 :`B` 1.0 :`A` 1.0) 14.0)
  (`KismetSystemLibrary.PrintString` "Updating the other widget" true false (struct :`R` 0.772115 :`B` 1.0 :`A` 1.0) 20.0)
  (bind _asi_siege_aim (cast `/Game/Mods/TDIRPAssets/Widgets/I_Siege_Aim` (`WidgetComponent.GetUserWidgetObject` (`self.NewWidget`))))
  (message `/Game/Mods/TDIRPAssets/Widgets/I_Siege_Aim.UpdateText` (`KismetSystemLibrary.Conv_InterfaceToObject` _asi_siege_aim) `Display Text`)
  (`KismetSystemLibrary.PrintString` "Didn't crash" true false)
  (`WidgetComponent.RequestRedraw` (`self.NewWidget`)))

(fn `UserConstructionScript`
  (`parent.UserConstructionScript`))